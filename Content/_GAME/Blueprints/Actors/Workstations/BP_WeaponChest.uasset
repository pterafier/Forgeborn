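; Weapon chest workstation that stores the player's finished crafted items and opens an inventory menu when interacted with empty-handed.
; Interact accepts equipped items with allowed IDs, and EvaluateItemState rejects those still needing quenching or sharpening with an action-log alert.
; UpdateItemDetails copies the forge state into the item struct, which goes into the Inventory before the held actor is destroyed.
; The cast item reference is cached and cleared only after a successful deposit.
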(event EventInteract
  (bind _playercharacter (Variables|Default|GetPlayerCharacter))
  (bind _playercontrollerbase (Variables|/Script/Forgeborn.PlayerCharacter|GetPlayerControllerBase _playercharacter))
  (bind _mainwidget (Variables|/Script/Forgeborn.PlayerControllerBase|GetMainWidget _playercontrollerbase))
  (Utilities|IsValid (Variables|/Script/Forgeborn.PlayerCharacter|GetEquippedItem (Variables|Default|GetPlayerCharacter))
    (:Is%20Valid
      (if (Utilities|Array|ContainsItem (Variables|Default|GetAcceptableItemIds) (.Id (Utilities|Struct|BreakItem (Variables|/Script/Forgeborn.ItemBase|GetItem (Variables|/Script/Forgeborn.PlayerCharacter|GetEquippedItem (Variables|Default|GetPlayerCharacter))))))
        (Utilities|IsValid (Variables|Default|GetAs%20BP%20Item)
          (:Is%20Valid
            _)
          (:Is%20Not%20Valid
            (bind _asbp_item (Utilities|Casting|CastToBP_Item (Variables|/Script/Forgeborn.PlayerCharacter|GetEquippedItem (Variables|Default|GetPlayerCharacter))))
            (Variables|Default|SetAs%20BP%20Item _asbp_item)))
        (bind _cancontinue (CallFunction|EvaluateItemState))
        (if _cancontinue
          (bind _updateditem (CallFunction|UpdateItemDetails))
          (Class|InventoryComponent|Add (Variables|Default|GetInventory) _updateditem 1)
          (Audio|PlaySound2D "/Game/_GAME/Audio/WAVs/Chest_Close.Chest_Close" 1.0 1.0 0.0 0 0)
          (CallFunction|AddEntrytoActionLog (Utilities|Text|FormatText "<Item>{item name}</> added to <Workstation>Item Chest</>" (.Name (Utilities|Struct|BreakItem (Variables|/Script/Forgeborn.ItemBase|GetItem (Variables|/Script/Forgeborn.PlayerCharacter|GetEquippedItem (Variables|Default|GetPlayerCharacter)))))))
          (Actor|DestroyActor (Variables|/Script/Forgeborn.PlayerCharacter|GetEquippedItem (Variables|Default|GetPlayerCharacter)))
          (Class|PlayerCharacter|SetEquippedItem (Variables|Default|GetPlayerCharacter))
          (Variables|Default|SetAs%20BP%20Item 0))))
    (:Is%20Not%20Valid
      (bind _returnvalue (Class|MainWidget|PushWidgettoTargetStack _mainwidget (Variables|/Script/Forgeborn.MainWidget|GetMenu_Stack _mainwidget) "/Game/_GAME/UI/Widgets/Inventory/Widgets/WB_GenericInventory.WB_GenericInventory_C" true false false))
      (bind _aswb_generic_inventory (Utilities|Casting|CastToWB_GenericInventory _returnvalue))
      (Default|SetOwningActor _aswb_generic_inventory self true)
      (Audio|PlaySound2D "/Game/_GAME/Audio/WAVs/Chest_Open.Chest_Open" 1.0 1.0 0.0 0 0))))

(fn ConstructionScript
  (|CallParentFunction))

(fn EvaluateItemState
  (bind _as_bp_item (Variables|Default|GetAs%20BP%20Item))
  (bind _item (Variables|/Script/Forgeborn.ItemBase|GetItem _as_bp_item))
  (bind (_id _name _description _transformsafterreachingtargettemperature _targettransformationtemperature _takesdamage _damagetemperature _maxtemperature _transformsinto_datatablerowname _requiresquenching _requiressharpening) (Utilities|Struct|BreakItem _item))
  (if _requiresquenching
    (switch Utilities|FlowControl|Switch|SwitchonEForgeState (Variables|/Game/_GAME/Blueprints/Actors/Items/BP_Item.BP_Item_C|GetItemProgressState (Variables|Default|GetAs%20BP%20Item))
      (:None
        (LocalVariables|SetisQuenched false :!label _label))
      (:Cool
        (goto _label))
      (:Hot
        (goto _label))
      (:Cooling
        (goto _label))
      (:Heating
        (goto _label))
      (:Ingot
        (goto _label))
      (:ShapingInProgress
        (goto _label))
      (:Shaped
        (goto _label))
      (:Quenched
        (LocalVariables|SetisQuenched true :!label _label_2))
      (:Tempered
        (goto _label_2))
      (:Sharpened
        (goto _label_2)))
    (if _requiressharpening
      (switch Utilities|FlowControl|Switch|SwitchonEForgeState (Variables|/Game/_GAME/Blueprints/Actors/Items/BP_Item.BP_Item_C|GetItemProgressState (Variables|Default|GetAs%20BP%20Item))
        (:None
          (LocalVariables|SetisSharpened false :!label _label_3))
        (:Cool
          (goto _label_3))
        (:Hot
          (goto _label_3))
        (:Cooling
          (goto _label_3))
        (:Heating
          (goto _label_3))
        (:Ingot
          (goto _label_3))
        (:ShapingInProgress
          (goto _label_3))
        (:Shaped
          (goto _label_3))
        (:Quenched
          (goto _label_3))
        (:Tempered
          (goto _label_3))
        (:Sharpened
          (LocalVariables|SetisSharpened true)))
      (if (LocalVariables|GetisSharpened)
        (return true)
        (else
          (CallFunction|AddEntrytoActionLog (Utilities|Text|FormatText "<Item>{item name}</> <Alert>needs to be sharpened!</>" _name))
          (return false)))
      (elif (LocalVariables|GetisQuenched)
        (return true)
        (else
          (CallFunction|AddEntrytoActionLog (Utilities|Text|FormatText "<Item>{item name}</> <Alert>needs to be quenched!</>" _name))
          (return false))))
    (else
      (return true))))

(fn UpdateItemDetails
  (bind _playercharacter (Variables|Default|GetPlayerCharacter))
  (bind _equippeditem (Variables|/Script/Forgeborn.PlayerCharacter|GetEquippedItem _playercharacter))
  (bind _item (Variables|/Script/Forgeborn.ItemBase|GetItem _equippeditem))
  (bind (_id _name _description _transformsafterreachingtargettemperature _targettransformationtemperature _takesdamage _damagetemperature _maxtemperature _transformsinto_datatablerowname _requiresquenching _requiressharpening _finalquality _maxquality _type _ore _maxstacksize _isvalid _icon _mesh _enchantmentniagarasystem) (Utilities|Struct|BreakItem _item))
  (bind _structout (Utilities|Struct|SetmembersinItem _item _id _name _description _requiresquenching _requiressharpening _finalquality _isvalid _icon _mesh _enchantmentniagarasystem (Variables|/Game/_GAME/Blueprints/Actors/Items/BP_Item.BP_Item_C|GetItemProgressState (Variables|Default|GetAs%20BP%20Item))))
  (return _structout))