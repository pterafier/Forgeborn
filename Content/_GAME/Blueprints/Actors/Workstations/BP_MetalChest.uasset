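; BP_MetalChest is an interactable workstation stockpile for one item type, identified by ItemId in DT_Items.
; Interacting while holding a matching item deposits it; empty-handed interaction spawns a BP_Item attached to the player's WeaponSocket, unless locked.
; Only items in IngotNamesArray are counted and limited by stock, shown on a counter widget; other items dispense without limit.
; Transfers and failed withdrawals are written to the action log.
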(event EventBeginPlay
  (bind _returnvalue (Actor|GetActorOfClass "/Game/_GAME/Blueprints/Actors/Managers/BP_ResourceManager.BP_ResourceManager_C"))
  (Variables|Default|SetResourceManager _returnvalue)
  (Development|SetHiddeninGame (Variables|Default|GetItemCountWidget) (Variables|Properties|GetHideItemCounter) false)
  (bind _aswb_interact_popup (Utilities|Casting|CastToWB_InteractPopup (UserInterface|GetWidget (Variables|Default|GetPopupWidgetComponent))))
  (Rendering|Components|TextRender|SetText (Variables|/Game/_GAME/UI/Widgets/HUD/Interaction/WB_InteractPopup.WB_InteractPopup_C|GetTXT_ActionText _aswb_interact_popup) (Utilities|Text|FormatText "{item} stockpile" (Variables|Default|GetActorName))))

(event EventInteract
  (bind _playercharacter (Variables|Default|GetPlayerCharacter))
  (bind _equippeditem (Variables|/Script/Forgeborn.PlayerCharacter|GetEquippedItem _playercharacter))
  (Utilities|IsValid _equippeditem
    (:Is%20Valid
      (CallFunction|AddHeldItemtoChest _equippeditem))
    (:Is%20Not%20Valid
      (if (not (Variables|Default|GetisLocked))
        (CallFunction|SpawnNewItem)
        (else
          (bind _returnvalue (CallFunction|FindItem (Variables|Properties|GetItemId)))
          (CallFunction|AddEntrytoActionLog (Utilities|Text|FormatText "<Workstation>{item name} Stockpile</><Alert> is locked!</>" (.Name (Utilities|Struct|BreakItem _returnvalue)))))))))

(fn ConstructionScript)

(fn AddHeldItemtoChest
  (params (Item :type Item%20Base%20Object%20Reference))
  (bind _newore (Variables|Default|GetNewOre))
  (bind (_id _name) (Utilities|Struct|BreakItem (Variables|/Script/Forgeborn.ItemBase|GetItem Item)))
  (if (== _id (Variables|Properties|GetItemId))
    (Class|PlayerCharacter|SetEquippedItem (Variables|Default|GetPlayerCharacter))
    (CallFunction|AddEntrytoActionLog (Utilities|Text|FormatText "<Item>{item name}</> added to <Workstation>{item name} Stockpile</>" _name))
    (if (Utilities|Array|ContainsItem (Variables|Default|GetIngotNamesArray) (.Name (Utilities|Struct|BreakItem (Variables|/Script/Forgeborn.ItemBase|GetItem Item))))
      (CallFunction|IncrementIngotCounter))
    (Utilities|IsValid _newore
      (:Is%20Valid
        (Actor|DestroyActor _newore)))))

(fn SpawnNewItem
  (bind _returnvalue (CallFunction|FindItem (Variables|Properties|GetItemId)))
  (LocalVariables|SetFoundItem _returnvalue)
  (if (Utilities|Array|ContainsItem (Variables|Default|GetIngotNamesArray) (.Name (Utilities|Struct|BreakItem _returnvalue)))
    (bind _success (CallFunction|TryDecrementIngotCounter))
    (if _success
      (bind _returnvalue_2 (Game|SpawnActorfromClass "/Game/_GAME/Blueprints/Actors/Items/BP_Item.BP_Item_C" (Transformation|GetWorldTransform (Variables|Default|GetSpawnPoint)) "Undefined" "MultiplyWithRoot" 0 (Variables|Default|GetPlayerCharacter) :!label _label))
      (bind _output_get (Variables|Default|SetNewOre _returnvalue_2))
      (Class|ItemBase|SetItem _output_get (LocalVariables|GetFoundItem))
      (Components|SkeletalMesh|SetSkeletalMeshAsset (Variables|/Script/Forgeborn.ItemBase|GetSkeletalMeshComponent (Variables|Default|GetNewOre)) (.Mesh (Utilities|Struct|BreakItem (LocalVariables|GetFoundItem))))
      (Transformation|AttachComponentToComponent (Variables|Default|GetNewOre) (Variables|/Script/Engine.Character|GetMesh (Variables|Default|GetPlayerCharacter)) "WeaponSocket" "SnapToTarget" "SnapToTarget" "SnapToTarget" true)
      (Class|PlayerCharacter|SetEquippedItem (Variables|Default|GetPlayerCharacter) (Variables|Default|GetNewOre))
      (CallFunction|AddEntrytoActionLog (Utilities|Text|FormatText "<Item>{item name}</> removed from <Workstation>{item name} Stockpile</>" (.Name (Utilities|Struct|BreakItem (LocalVariables|GetFoundItem)))))
      (Audio|PlaySound2D "/Game/_GAME/Audio/WAVs/Footstep_Land_v1.Footstep_Land_v1" 1.0 1.0 0.0 0 0)
      (else
        (CallFunction|AddEntrytoActionLog (Utilities|Text|FormatText "<Workstation>{item name} Stockpile</><Alert> doesn't have any </><Item>{item name}!</>" (.Name (Utilities|Struct|BreakItem (Variables|/Script/Forgeborn.ItemBase|GetItem (Variables|Default|GetNewOre))))))))
    (else
      (goto _label))))

(fn TryDecrementIngotCounter
  (if (> (Variables|Default|GetItemCount) 0)
    (Math|Integer|DecrementInt (Variables|Default|GetItemCount)
      (:%20%20
        (CallFunction|UpdateItemCountText)
        (return true)))
    (else
      (return false))))

(fn IncrementIngotCounter
  (Math|Integer|IncrementInt (Variables|Default|GetItemCount)
    (:%20%20
      (CallFunction|UpdateItemCountText))))

(fn UpdateItemCountText
  (Utilities|IsValid (Variables|Default|GetAs%20WB%20Item%20Counter)
    (:Is%20Valid
      _)
    (:Is%20Not%20Valid
      (bind _aswb_item_counter (Utilities|Casting|CastToWB_ItemCounter (UserInterface|GetWidget (Variables|Default|GetItemCountWidget))))
      (Variables|Default|SetAs%20WB%20Item%20Counter _aswb_item_counter)))
  (Default|UpdateItemText (Variables|Default|GetAs%20WB%20Item%20Counter) (Utilities|Text|ToText(Integer) (Variables|Default|GetItemCount))))

(fn FindItem
  (params (Id :type Integer))
  (bind _returnvalue (Utilities|GetDataTableRow "/Game/_GAME/Data/DT_Items.DT_Items" (Utilities|String|StringToName (Utilities|String|ToString(Integer) Id)))
    (:then
      _)
    (:RowNotFound
      _))
  (return _returnvalue))