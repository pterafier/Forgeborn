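; Anvil workstation actor where the player shapes a sufficiently hot, accepted item through a minigame.
; Interact snaps the equipped item onto the anvil, shows the hammer and hides temperature widgets; exiting returns the item to the weapon socket.
; The minigame score feeds UpdatePlayerItem, which swaps in the shaped item's DataTable row, resets temperature and adds clamped quality.
; Items needing no quenching or sharpening receive their final quality there.
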(event Custom|OnMinigameComplete_Event
  (params (FinalScore :type Integer) (TotalPointsPossible :type Integer))
  (CallFunction|UpdatePlayerItem (* (/ FinalScore TotalPointsPossible) 8e+01)))

(event EventInteract
  (bind _playercharacter (Variables|Default|GetPlayerCharacter))
  (bind _playercharacter_2 (Variables|Default|GetPlayerCharacter))
  (bind _playercharacter_3 (Variables|Default|GetPlayerCharacter))
  (bind _equippeditem (Variables|/Script/Forgeborn.PlayerCharacter|GetEquippedItem _playercharacter))
  (bind _equippeditem_2 (Variables|/Script/Forgeborn.PlayerCharacter|GetEquippedItem _playercharacter_2))
  (bind _item (Variables|/Script/Forgeborn.ItemBase|GetItem _equippeditem_2))
  (bind _temperaturecomponent (Variables|/Script/Forgeborn.ItemBase|GetTemperatureComponent _equippeditem))
  (bind (_id _name) (Utilities|Struct|BreakItem _item))
  (Utilities|IsValid (Variables|/Script/Forgeborn.PlayerCharacter|GetEquippedItem (Variables|Default|GetPlayerCharacter))
    (:Is%20Valid
      (if (Utilities|Array|ContainsItem (Variables|Default|GetAcceptableItemIds) _id)
        (if (>= (Variables|/Script/Forgeborn.TemperatureComponent|GetTemperature _temperaturecomponent) (Variables|/Script/Forgeborn.TemperatureComponent|GetRequiredTemperatureForShaping _temperaturecomponent))
          (Transformation|DetachFromActor (Variables|/Script/Forgeborn.PlayerCharacter|GetEquippedItem (Variables|Default|GetPlayerCharacter)) "KeepWorld" "KeepWorld" "KeepWorld")
          (Transformation|AttachComponentToComponent (Variables|/Script/Forgeborn.PlayerCharacter|GetEquippedItem (Variables|Default|GetPlayerCharacter)) (Variables|Default|GetItemArrow) "None" "SnapToTarget" "SnapToTarget" "SnapToTarget" true)
          (|CallParentFunction)
          (Default|HideTemperatureWidget (Variables|Default|GetForgeRef) true)
          (Utilities|IsValid (Variables|Default|GetAs%20BP%20Item)
            (:Is%20Valid
              _)
            (:Is%20Not%20Valid
              (bind _asbp_item (Utilities|Casting|CastToBP_Item (Variables|/Script/Forgeborn.PlayerCharacter|GetEquippedItem (Variables|Default|GetPlayerCharacter))))
              (Variables|Default|SetAs%20BP%20Item _asbp_item)))
          (Development|SetHiddeninGame (Variables|/Game/_GAME/Blueprints/Actors/Items/BP_Item.BP_Item_C|GetTempWidget (Variables|Default|GetAs%20BP%20Item)) true false)
          (Class|PlayerCharacter|HideHammer _playercharacter_3 false)
          (Variables|/Script/Forgeborn.PlayerCharacter|SetAtAnvil _playercharacter_3 true)
          (Audio|PlaySound2D "/Game/_GAME/Audio/WAVs/Hit_Marker_V4_3_.Hit_Marker_V4_3_" 1.0 1.0 0.0 0 0)
          (else
            (CallFunction|AddEntrytoActionLog (Utilities|Text|FormatText "<Item>{item name}</><Alert> isn't hot enough!</>" _name))))))))

(event EventOnPlayerExitWorkstation
  (bind _playercharacter (Variables|Default|GetPlayerCharacter))
  (Transformation|DetachFromActor (Variables|/Script/Forgeborn.PlayerCharacter|GetEquippedItem (Variables|Default|GetPlayerCharacter)) "KeepWorld" "KeepWorld" "KeepWorld")
  (Transformation|AttachComponentToComponent (Variables|/Script/Forgeborn.PlayerCharacter|GetEquippedItem _playercharacter) (Variables|/Script/Engine.Character|GetMesh _playercharacter) "WeaponSocket" "SnapToTarget" "SnapToTarget" "SnapToTarget" true)
  (Class|PlayerCharacter|HideHammer (Variables|Default|GetPlayerCharacter) true)
  (Default|HideTemperatureWidget (Variables|Default|GetForgeRef) false)
  (Variables|/Script/Forgeborn.PlayerCharacter|SetAtAnvil (Variables|Default|GetPlayerCharacter) false))

(event EventOnMinigameWidgetActivated
  (bind _minigamewidgetinstance (Variables|Default|GetMinigameWidgetInstance))
  (Utilities|IsValid _minigamewidgetinstance
    (:Is%20Valid
      (bind _aswb_minigame_widget (Utilities|Casting|CastToWB_MinigameWidget _minigamewidgetinstance))
      (EventDispatchers|UnbindallEventsfromOnMinigameComplete _aswb_minigame_widget) ; For safety so we don't bind multiple times
      (EventDispatchers|AssignOnMinigameComplete _aswb_minigame_widget (delegate Custom|OnMinigameComplete_Event)))))

(event EventBeginPlay
  (|CallParentFunction)
  (CallFunction|SetReferences))

(fn ConstructionScript)

(fn UpdatePlayerItem
  (params (QualityScore :type Float%20%28double-precision%29))
  (bind _playercharacter (Variables|Default|GetPlayerCharacter))
  (bind _equippeditem (Variables|/Script/Forgeborn.PlayerCharacter|GetEquippedItem _playercharacter))
  (LocalVariables|SetOldItemName (.Name (Utilities|Struct|BreakItem (Variables|/Script/Forgeborn.ItemBase|GetItem (Variables|/Script/Forgeborn.PlayerCharacter|GetEquippedItem (Variables|Default|GetPlayerCharacter))))))
  (bind _returnvalue (Utilities|GetDataTableRow "/Game/_GAME/Data/DT_Items.DT_Items" (Utilities|String|StringToName (Utilities|String|ToString(Integer) (Variables|Default|GetCurrentItemId))))
    (:then
      (Class|ItemBase|SetItem _equippeditem _returnvalue)
      (Components|SkeletalMesh|SetSkeletalMeshAsset (Variables|/Script/Forgeborn.ItemBase|GetSkeletalMeshComponent _equippeditem) (.Mesh (Utilities|Struct|BreakItem _returnvalue)))
      (bind _asbp_item (Utilities|Casting|CastToBP_Item (Variables|/Script/Forgeborn.PlayerCharacter|GetEquippedItem (Variables|Default|GetPlayerCharacter))))
      (Default|ResetItemTemperature _asbp_item)
      (Variables|/Game/_GAME/Blueprints/Actors/Items/BP_Item.BP_Item_C|SetItemProgressState _asbp_item "Shaped")
      (Variables|/Game/_GAME/Blueprints/Actors/Items/BP_Item.BP_Item_C|SetQuality _asbp_item (Math|Float|Clamp(Float) (+ (Variables|/Game/_GAME/Blueprints/Actors/Items/BP_Item.BP_Item_C|GetQuality _asbp_item) QualityScore) 0.0 (.MaxQuality (Utilities|Struct|BreakItem _returnvalue))))
      (CallFunction|AddEntrytoActionLog (Utilities|Text|FormatText "<Item>{old item name}</> successfully shaped into <Item>{new item}</>" (LocalVariables|GetOldItemName) (.Name (Utilities|Struct|BreakItem _returnvalue))))
      (if (and (not (.RequiresQuenching (Utilities|Struct|BreakItem _returnvalue))) (not (.RequiresSharpening (Utilities|Struct|BreakItem _returnvalue))))
        (bind _returnvalue_2 (Class|ItemBase|GetItemQuality (Variables|/Script/Forgeborn.PlayerCharacter|GetEquippedItem (Variables|Default|GetPlayerCharacter)) (* (/ (Variables|/Game/_GAME/Blueprints/Actors/Items/BP_Item.BP_Item_C|GetQuality _asbp_item) (.MaxQuality (Utilities|Struct|BreakItem _returnvalue))) 5.0)))
        (CallFunction|AddEntrytoActionLog (Utilities|Text|FormatText "<Item>{New Item Name}</> complete. Final Quality: <{Quality}>{Quality}</>" (.Name (Utilities|Struct|BreakItem _returnvalue)) (|GenerictoText _returnvalue_2)))
        (Development|SetHiddeninGame (Variables|/Game/_GAME/Blueprints/Actors/Items/BP_Item.BP_Item_C|GetTempWidget _asbp_item) true false)
        (Utilities|Struct|SetmembersinItem (Variables|/Script/Forgeborn.ItemBase|GetItem (Variables|/Script/Forgeborn.PlayerCharacter|GetEquippedItem (Variables|Default|GetPlayerCharacter))) _returnvalue_2)
        (CallFunction|PlayFinishedQualitySound _returnvalue_2)
        (else
          (Utilities|IsValid (Variables|Default|GetAs%20BP%20Item)
            (:Is%20Valid
              _)
            (:Is%20Not%20Valid
              (bind _asbp_item_2 (Utilities|Casting|CastToBP_Item (Variables|/Script/Forgeborn.PlayerCharacter|GetEquippedItem (Variables|Default|GetPlayerCharacter))))
              (Variables|Default|SetAs%20BP%20Item _asbp_item_2)))
          (Development|SetHiddeninGame (Variables|/Game/_GAME/Blueprints/Actors/Items/BP_Item.BP_Item_C|GetTempWidget (Variables|Default|GetAs%20BP%20Item)) false false))))))

(fn SetReferences
  (bind _returnvalue (Actor|GetActorOfClass "/Game/_GAME/Blueprints/Actors/Workstations/BP_Forge.BP_Forge_C"))
  (Variables|Default|SetForgeRef _returnvalue))