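; Quench tank workstation where the player quenches a held item, then retrieves it by interacting again.
; Adding grades item temperature against its transformation and damage thresholds as perfect, too hot or too cool.
; Perfect and too-hot items become Quenched, with a quality penalty for too hot; those not needing sharpening get a final quality.
; Too-cool items stay unquenched but still enter the tank and have their temperature reset.
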(event EventBeginPlay
  (|CallParentFunction))

(event EventInteract
  (switch Utilities|FlowControl|Switch|SwitchonEWorkstationAction (Variables|Default|GetWorkstationAction)
    (:Add
      (CallFunction|AddItemtoWorkstation))
    (:Remove
      (CallFunction|RemoveItemfromWorkstation))))

(fn ConstructionScript)

(fn IsItemTemperatureHighEnough
  (return (>= (Variables|/Script/Forgeborn.TemperatureComponent|GetTemperature (Variables|/Script/Forgeborn.ItemBase|GetTemperatureComponent (Variables|/Script/Forgeborn.PlayerCharacter|GetEquippedItem (Variables|Default|GetPlayerCharacter)))) (.TargetTransformationTemperature (Utilities|Struct|BreakItem (Variables|/Script/Forgeborn.ItemBase|GetItem (Variables|/Script/Forgeborn.PlayerCharacter|GetEquippedItem (Variables|Default|GetPlayerCharacter))))))))

(fn IsItemTakingDamage
  (return (>= (Variables|/Script/Forgeborn.TemperatureComponent|GetTemperature (Variables|/Script/Forgeborn.ItemBase|GetTemperatureComponent (Variables|/Script/Forgeborn.PlayerCharacter|GetEquippedItem (Variables|Default|GetPlayerCharacter)))) (.DamageTemperature (Utilities|Struct|BreakItem (Variables|/Script/Forgeborn.ItemBase|GetItem (Variables|/Script/Forgeborn.PlayerCharacter|GetEquippedItem (Variables|Default|GetPlayerCharacter))))))))

(fn SetItemStateQuenched
  (params (QuenchResult :type EQuenchResult%20Enum :default "None"))
  (switch Utilities|FlowControl|Switch|SwitchonEQuenchResult QuenchResult
    (:Perfect
      (Class|ItemBase|SetItemState (Variables|/Script/Forgeborn.PlayerCharacter|GetEquippedItem (Variables|Default|GetPlayerCharacter)) "Quenched" :!label _label)
      (Variables|/Game/_GAME/Blueprints/Actors/Items/BP_Item.BP_Item_C|SetItemProgressState (Variables|Default|GetCurrentItem) "Quenched"))
    (:TooHot
      (goto _label))
    (:TooCool
      (CallFunction|AddEntrytoActionLog (Utilities|Text|FormatText "<Item>{item name}</><Alert> too cool to quench!</>" (.Name (Utilities|Struct|BreakItem (Variables|/Script/Forgeborn.ItemBase|GetItem (Variables|/Script/Forgeborn.PlayerCharacter|GetEquippedItem (Variables|Default|GetPlayerCharacter))))))))))

(fn EvaluateQuenchResult
  (if (and (CallFunction|IsItemTemperatureHighEnough) (not (CallFunction|IsItemTakingDamage)))
    (CallFunction|SetItemStateQuenched "Perfect")
    (Variables|Default|SetQuenchResult "Perfect")
    (elif (CallFunction|IsItemTakingDamage)
      (CallFunction|SetItemStateQuenched "TooHot")
      (Variables|Default|SetQuenchResult "TooHot")
      (else
        (CallFunction|SetItemStateQuenched "TooCool")
        (Variables|Default|SetQuenchResult "TooCool")))))

(fn UpdateLogwithQuenchResult
  (bind _currentitem (Variables|Default|GetCurrentItem))
  (bind _item (Variables|/Script/Forgeborn.ItemBase|GetItem _currentitem))
  (bind _name (Utilities|Struct|BreakItem _item))
  (switch Utilities|FlowControl|Switch|SwitchonEQuenchResult (Variables|Default|GetQuenchResult)
    (:Perfect
      (CallFunction|AddEntrytoActionLog (Utilities|Text|FormatText "<Item>{item name}</><Perfect> quenched perfectly!</>" _name)))
    (:TooHot
      (CallFunction|AddEntrytoActionLog (Utilities|Text|FormatText "<Perfect>Quench succeeded.</> <Item>{item name}</><Alert> too hot!</>" _name)))
    (:TooCool
      (CallFunction|AddEntrytoActionLog (Utilities|Text|FormatText "<Alert>Quench failed! </><Item>{item name}</><Alert> too cool to quench!</>" _name)))))

(fn AddItemtoWorkstation
  (bind _playercharacter (Variables|Default|GetPlayerCharacter))
  (bind _equippeditem (Variables|/Script/Forgeborn.PlayerCharacter|GetEquippedItem _playercharacter))
  (bind _item (Variables|/Script/Forgeborn.ItemBase|GetItem _equippeditem))
  (bind (_id _name) (Utilities|Struct|BreakItem _item))
  (if (Variables|Default|GetisAcceptingItems)
    (Utilities|IsValid (Variables|Default|GetCurrentItem)
      (:Is%20Valid
        _)
      (:Is%20Not%20Valid
        (bind _asbp_item (Utilities|Casting|CastToBP_Item (Variables|/Script/Forgeborn.PlayerCharacter|GetEquippedItem (Variables|Default|GetPlayerCharacter))))
        (Variables|Default|SetCurrentItem _asbp_item)))
    (if (Utilities|Array|ContainsItem (Variables|Default|GetAcceptableItemIds) _id)
      (switch Utilities|FlowControl|Switch|SwitchonEForgeState (Variables|/Game/_GAME/Blueprints/Actors/Items/BP_Item.BP_Item_C|GetItemProgressState (Variables|Default|GetCurrentItem))
        (:None
          (CallFunction|EvaluateQuenchResult :!label _label)
          (if (Utilities|Enum|Equal(Enum) (Variables|/Game/_GAME/Blueprints/Actors/Items/BP_Item.BP_Item_C|GetItemProgressState (Variables|Default|GetCurrentItem)) "Quenched")
            (Default|ResetItemTemperature (Variables|Default|GetCurrentItem))
            (CallFunction|UpdateLogwithQuenchResult)
            (CallFunction|UpdateItemQualityfromQuenchResult)
            (Transformation|DetachFromActor (Variables|/Script/Forgeborn.PlayerCharacter|GetEquippedItem (Variables|Default|GetPlayerCharacter)) "KeepWorld" "KeepWorld" "KeepWorld")
            (Transformation|AttachComponentToComponent (Variables|/Script/Forgeborn.PlayerCharacter|GetEquippedItem (Variables|Default|GetPlayerCharacter)) (Variables|Default|GetArrow) "None" "SnapToTarget" "SnapToTarget" "SnapToTarget" true)
            (Transformation|SetWorldRotation (Variables|/Script/Engine.Actor|GetRootComponent (Variables|/Script/Forgeborn.PlayerCharacter|GetEquippedItem (Variables|Default|GetPlayerCharacter))) (Transformation|GetWorldRotation (Variables|Default|GetArrow)) false false)
            (Class|PlayerCharacter|SetEquippedItem (Variables|Default|GetPlayerCharacter))
            (CallFunction|SetWorkstationAction "Remove" false)
            (Audio|PlaySound2D "/Game/_GAME/Audio/WAVs/Quench_QTE_SFX_v1.Quench_QTE_SFX_v1" 1.0 1.0 0.0 0 0)
            (Niagara|SpawnSystematLocation "/Game/AmtosphericFX/FX/NS_Fire_Medium.NS_Fire_Medium" (Transformation|GetWorldLocation (Variables|Default|GetArrow)))
            (Audio|PlaySound2D "/Game/_GAME/Audio/WAVs/534702__plasterbrain__lighting-a-fire.534702__plasterbrain__lighting-a-fire" 0.8 0.8 0.0 0 0)
            (if (not (.RequiresSharpening (Utilities|Struct|BreakItem (Variables|/Script/Forgeborn.ItemBase|GetItem (Variables|Default|GetCurrentItem)))))
              (bind _returnvalue (Class|ItemBase|GetItemQuality (Variables|Default|GetCurrentItem) (* (/ (Variables|/Game/_GAME/Blueprints/Actors/Items/BP_Item.BP_Item_C|GetQuality (Variables|Default|GetCurrentItem)) (.MaxQuality (Utilities|Struct|BreakItem (Variables|/Script/Forgeborn.ItemBase|GetItem (Variables|Default|GetCurrentItem))))) 5.0)))
              (CallFunction|AddEntrytoActionLog (Utilities|Text|FormatText "<Item>{item name}</> complete. Final Quality: <{Quality}>{Quality}</>" (.Name (Utilities|Struct|BreakItem (Variables|/Script/Forgeborn.ItemBase|GetItem (Variables|Default|GetCurrentItem)))) (|GenerictoText _returnvalue)))
              (Development|SetHiddeninGame (Variables|/Game/_GAME/Blueprints/Actors/Items/BP_Item.BP_Item_C|GetTempWidget (Variables|Default|GetCurrentItem)) true false)
              (Utilities|Struct|SetmembersinItem (Variables|/Script/Forgeborn.ItemBase|GetItem (Variables|Default|GetCurrentItem)) _returnvalue)
              (CallFunction|PlayFinishedQualitySound _returnvalue))
            (else
              (Default|ResetItemTemperature (Variables|Default|GetCurrentItem))
              (Transformation|DetachFromActor (Variables|/Script/Forgeborn.PlayerCharacter|GetEquippedItem (Variables|Default|GetPlayerCharacter)) "KeepWorld" "KeepWorld" "KeepWorld")
              (Transformation|AttachComponentToComponent (Variables|/Script/Forgeborn.PlayerCharacter|GetEquippedItem (Variables|Default|GetPlayerCharacter)) (Variables|Default|GetArrow) "None" "SnapToTarget" "SnapToTarget" "SnapToTarget" true)
              (Transformation|SetWorldRotation (Variables|/Script/Engine.Actor|GetRootComponent (Variables|/Script/Forgeborn.PlayerCharacter|GetEquippedItem (Variables|Default|GetPlayerCharacter))) (Transformation|GetWorldRotation (Variables|Default|GetArrow)) false false)
              (Class|PlayerCharacter|SetEquippedItem (Variables|Default|GetPlayerCharacter))
              (CallFunction|SetWorkstationAction "Remove" false))))
        (:Cool
          (goto _label))
        (:Hot
          (goto _label))
        (:Cooling
          (goto _label))
        (:Heating
          (goto _label))
        (:Ingot
          (goto _label))
        (:ShapingInProgress
          (goto _label))
        (:Shaped
          (goto _label))
        (:Quenched
          (CallFunction|AddEntrytoActionLog (Utilities|Text|FormatText "<Item>{item name}</><Alert> already quenched!</>" _name) :!label _label_2))
        (:Tempered
          (goto _label_2))
        (:Sharpened
          (goto _label_2))))))

(fn SetWorkstationAction
  (params (Workstation%20Action :type EWorkstationAction%20Enum :default "None") (Is%20Accepting%20Items :type Boolean))
  (Variables|Default|SetWorkstationAction Workstation%20Action)
  (Variables|Default|SetisAcceptingItems Is%20Accepting%20Items))

(fn RemoveItemfromWorkstation
  (if (not (Utilities|IsValid (Variables|/Script/Forgeborn.PlayerCharacter|GetEquippedItem (Variables|Default|GetPlayerCharacter))))
    (Transformation|DetachFromActor (Variables|Default|GetCurrentItem) "KeepWorld" "KeepWorld" "KeepWorld")
    (Transformation|AttachComponentToComponent (Variables|Default|GetCurrentItem) (Variables|/Script/Engine.Character|GetMesh (Variables|Default|GetPlayerCharacter)) "WeaponSocket" "SnapToTarget" "SnapToTarget" "SnapToTarget" true)
    (Class|PlayerCharacter|SetEquippedItem (Variables|Default|GetPlayerCharacter) (Variables|Default|GetCurrentItem))
    (CallFunction|AddEntrytoActionLog (Utilities|Text|FormatText "<Item>{item name}</> removed from <Workstation>Quench Tank</>" (.Name (Utilities|Struct|BreakItem (Variables|/Script/Forgeborn.ItemBase|GetItem (Variables|Default|GetCurrentItem))))))
    (Variables|Default|SetCurrentItem 0)
    (CallFunction|SetWorkstationAction "Add" true)))

(fn UpdateItemQualityfromQuenchResult
  (bind _currentitem (Variables|Default|GetCurrentItem))
  (switch Utilities|FlowControl|Switch|SwitchonEQuenchResult (Variables|Default|GetQuenchResult)
    (:TooHot
      (Variables|/Game/_GAME/Blueprints/Actors/Items/BP_Item.BP_Item_C|SetQuality _currentitem (- (Variables|/Game/_GAME/Blueprints/Actors/Items/BP_Item.BP_Item_C|GetQuality _currentitem) 2e+01)))))