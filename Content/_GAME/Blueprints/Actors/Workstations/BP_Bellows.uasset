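; Bellows workstation actor that heats its linked forge for a limited time when interacted with.
; Each interaction extends the clamped heating duration, starts forge heating and resets the timer that triggers cooling on expiry.
; A looping timer at the forge's heating rate decays the bonus in proportion to time left.
; A frame-delta looping timer updates the widget progress bar and is never cleared, as those clear calls are unconnected.
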(event EventBeginPlay
  (|CallParentFunction)
  (bind _aswb_time_progress_bar (Utilities|Casting|CastToWB_TimeProgressBar (UserInterface|GetWidget (Variables|Default|GetTimeRemainingWidget))))
  (Variables|Default|SetAs%20WB%20Time%20Progress%20Bar _aswb_time_progress_bar)
  (CallFunction|UpdateTimerProgressBar))

(event EventInteract
  (bind _linkedforgeactor (Variables|Default|GetLinkedForgeActor))
  (bind _temperature (Variables|/Game/_GAME/Blueprints/Actors/Workstations/BP_Forge.BP_Forge_C|GetTemperature _linkedforgeactor))
  (Utilities|IsValid (Variables|Default|GetLinkedForgeActor)
    (:Is%20Valid
      (if (Variables|Default|GetCanPlaySound)
        (Audio|PlaySoundatLocation "/Game/_GAME/Audio/WAVs/SC_Bellow_Interact_v1_Cue.SC_Bellow_Interact_v1_Cue" (Transformation|GetActorLocation (Components|GetOwner (Variables|Default|GetStaticMeshComponent))) "0, 0, 0" 1.0 1.0 0.0 0 0 0 0)
        (Variables|Default|SetCanPlaySound true))
      (CallFunction|UpgradeHeatingDuration)
      (bind _returnvalue (Utilities|Time|SetTimerbyFunctionName 0 "TriggerForgeCooling" (Variables|Default|GetHeatingDuration)))
      (Variables|Default|SetForgeCoolingTimerHandle _returnvalue)
      (Class|TemperatureComponent|StartHeating _temperature)
      (bind _returnvalue_2 (Utilities|Time|SetTimerbyFunctionName 0 "ReduceBonusTime" (Variables|/Script/Forgeborn.TemperatureComponent|GetHeatingRate _temperature) true))
      (Variables|Default|SetBonusTimeReductionTimerHandle _returnvalue_2)
      (bind _returnvalue_3 (Utilities|Time|SetTimerbyFunctionName 0 "UpdateTimerProgressBar" (Utilities|Time|GetWorldDeltaSeconds) true))
      (Variables|Default|SetProgressBarTimerHandle _returnvalue_3))
    (:Is%20Not%20Valid
      (Development|PrintString "Bellows do not have a forge assigned!" true true "(R=1.000000,G=0.000000,B=0.000000,A=1.000000)" 1e+01))))

(fn ConstructionScript)

(fn ReduceBonusTime
  (Variables|Default|SetHeatingDuration (Math|Float|Clamp(Float) (- (Variables|Default|GetHeatingDuration) (* (Math|Float|SafeDivide (Utilities|Time|GetTimerRemainingTimebyHandle (Variables|Default|GetForgeCoolingTimerHandle)) (Variables|Default|GetMaxHeatingDuration)) 0.125)) (Variables|Default|GetMinHeatingDuration) (Variables|Default|GetMaxHeatingDuration)))
  (if (Math|Float|NearlyEqual(Float) (Math|Float|SafeDivide (Utilities|Time|GetTimerRemainingTimebyHandle (Variables|Default|GetForgeCoolingTimerHandle)) (Variables|Default|GetMaxHeatingDuration)) 0.0 0.01)
    (Utilities|Time|ClearandInvalidateTimerbyHandle (Variables|Default|GetBonusTimeReductionTimerHandle))
    (Variables|Default|SetHeatingDuration (Variables|Default|GetMinHeatingDuration))))

(fn UpgradeHeatingDuration
  (Variables|Default|SetHeatingDuration (Math|Float|Clamp(Float) (+ (Variables|Default|GetHeatingDuration) (Variables|Default|GetBonusHeatingDurationAmount)) (Variables|Default|GetMinHeatingDuration) (Variables|Default|GetMaxHeatingDuration)))
  (CallFunction|UpdateTimerProgressBar))

(fn TriggerForgeCooling
  (Class|TemperatureComponent|StartCooling (Variables|/Game/_GAME/Blueprints/Actors/Workstations/BP_Forge.BP_Forge_C|GetTemperature (Variables|Default|GetLinkedForgeActor)))
  (CallFunction|UpdateTimerProgressBar)
  (Development|PrintString "Cooling started"))

(fn UpdateTimerProgressBar
  (bind _as_wb_time_progress_bar (Variables|Default|GetAs%20WB%20Time%20Progress%20Bar))
  (bind _maxheatingduration (Variables|Default|GetMaxHeatingDuration))
  (bind _forgecoolingtimerhandle (Variables|Default|GetForgeCoolingTimerHandle))
  (bind _returnvalue (Utilities|Time|GetTimerRemainingTimebyHandle _forgecoolingtimerhandle))
  (bind _returnvalue_2 (Math|Float|SafeDivide _returnvalue _maxheatingduration))
  (Utilities|IsValid _as_wb_time_progress_bar
    (:Is%20Valid
      (Default|SetPercent _as_wb_time_progress_bar _returnvalue_2)
      (if (Math|Float|NearlyEqual(Float) _returnvalue_2 0.0 0.005)
        _))))

(fn ResetProgress
  (Utilities|Time|ClearandInvalidateTimerbyHandle (Variables|Default|GetForgeCoolingTimerHandle))
  (Utilities|Time|ClearandInvalidateTimerbyHandle (Variables|Default|GetBonusTimeReductionTimerHandle))
  (Variables|Default|SetHeatingDuration (Variables|Default|GetMinHeatingDuration))
  (CallFunction|ClearProgressBar))

(fn ClearProgressBar
  (bind _as_wb_time_progress_bar (Variables|Default|GetAs%20WB%20Time%20Progress%20Bar))
  (Utilities|IsValid _as_wb_time_progress_bar
    (:Is%20Valid
      (Default|SetPercent _as_wb_time_progress_bar 0.0))))