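; BP_GrindingWheel is a workstation where the player sharpens a quenched or tempered item through a minigame, finishing it with a final quality.
; Interact checks the equipped item's ID and progress state, then snaps it to the player's grinder socket and starts the wheel animation, sparks and audio, or logs why it refuses.
; Minigame completion adds score-scaled quality, marks the item Sharpened, logs and sounds the result, and undoes the grinding setup.
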(event Custom|OnMinigameComplete_Event
  (params (FinalScore :type Integer) (TotalPointsPossible :type Integer))
  (bind _currentitem (Variables|Default|GetCurrentItem))
  (bind _currentitem_2 (Variables|Default|GetCurrentItem))
  (bind _playercharacter (Variables|Default|GetPlayerCharacter))
  (bind _item (Variables|/Script/Forgeborn.ItemBase|GetItem _currentitem))
  (bind (_name _maxtemperature _requiresquenching _requiressharpening _finalquality _maxquality) (Utilities|Struct|BreakItem _item))
  (Variables|/Game/_GAME/Blueprints/Actors/Items/BP_Item.BP_Item_C|SetQuality _currentitem_2 (+ (Variables|/Game/_GAME/Blueprints/Actors/Items/BP_Item.BP_Item_C|GetQuality _currentitem_2) (* (/ FinalScore TotalPointsPossible) 3e+01)))
  (Variables|/Game/_GAME/Blueprints/Actors/Items/BP_Item.BP_Item_C|SetItemProgressState (Variables|Default|GetCurrentItem) "Sharpened")
  (bind _returnvalue (Class|ItemBase|GetItemQuality (Variables|Default|GetCurrentItem) (* (/ (Variables|/Game/_GAME/Blueprints/Actors/Items/BP_Item.BP_Item_C|GetQuality _currentitem) _maxquality) 5.0)))
  (CallFunction|AddEntrytoActionLog (Utilities|Text|FormatText "<Item>{item name}</> completed! Final Quality: <{quality}>{quality}</> " _name (|GenerictoText _returnvalue)))
  (Development|SetHiddeninGame (Variables|/Game/_GAME/Blueprints/Actors/Items/BP_Item.BP_Item_C|GetTempWidget (Variables|Default|GetCurrentItem)) true false)
  (Utilities|Struct|SetmembersinItem (Variables|/Script/Forgeborn.ItemBase|GetItem (Variables|Default|GetCurrentItem)) _returnvalue)
  (Variables|/Script/Engine.SkeletalMeshComponent|SetbPauseAnims (Variables|Default|GetSkeletalMesh) true)
  (Transformation|AttachComponentToComponent (Variables|/Script/Forgeborn.PlayerCharacter|GetEquippedItem _playercharacter) (Variables|/Script/Engine.Character|GetMesh _playercharacter) "WeaponSocket" "SnapToTarget" "SnapToTarget" "SnapToTarget" true)
  (Variables|/Script/Forgeborn.PlayerCharacter|SetAtGrindingWheel (Variables|Default|GetPlayerCharacter) false)
  (Components|DestroyComponent (Variables|Default|GetSparks))
  (CallFunction|PlayFinishedQualitySound _returnvalue)
  (Audio|Components|Audio|FadeOut (Variables|Default|GetAudioComponent) 0.5 0.0 "Linear" :!class /Script/Engine.AudioComponent))

(event EventBeginPlay
  (|CallParentFunction)
  (Audio|Components|Audio|Stop (Variables|Default|GetAudioComponent)))

(event EventInteract
  (bind _playercharacter (Variables|Default|GetPlayerCharacter))
  (Utilities|IsValid (Variables|/Script/Forgeborn.PlayerCharacter|GetEquippedItem (Variables|Default|GetPlayerCharacter))
    (:Is%20Valid
      (if (Utilities|Array|ContainsItem (Variables|Default|GetAcceptableItemIds) (.Id (Utilities|Struct|BreakItem (Variables|/Script/Forgeborn.ItemBase|GetItem (Variables|/Script/Forgeborn.PlayerCharacter|GetEquippedItem (Variables|Default|GetPlayerCharacter))))))
        (Utilities|IsValid (Variables|Default|GetCurrentItem)
          (:Is%20Valid
            _)
          (:Is%20Not%20Valid
            (bind _asbp_item (Utilities|Casting|CastToBP_Item (Variables|/Script/Forgeborn.PlayerCharacter|GetEquippedItem (Variables|Default|GetPlayerCharacter))))
            (Variables|Default|SetCurrentItem _asbp_item)))
        (switch Utilities|FlowControl|Switch|SwitchonEForgeState (Variables|/Game/_GAME/Blueprints/Actors/Items/BP_Item.BP_Item_C|GetItemProgressState (Variables|Default|GetCurrentItem))
          (:None
            (CallFunction|AddEntrytoActionLog (Utilities|Text|FormatText "<Item>{item name}</><Alert> not quenched!</>" (.Name (Utilities|Struct|BreakItem (Variables|/Script/Forgeborn.ItemBase|GetItem (Variables|Default|GetCurrentItem))))) :!label _label))
          (:Cool
            (goto _label))
          (:Hot
            (goto _label))
          (:Cooling
            (goto _label))
          (:Heating
            (goto _label))
          (:Ingot
            (goto _label))
          (:ShapingInProgress
            (goto _label))
          (:Shaped
            (goto _label))
          (:Quenched
            (|CallParentFunction :!label _label_2)
            (Variables|/Script/Engine.SkeletalMeshComponent|SetbPauseAnims (Variables|Default|GetSkeletalMesh) false)
            (Transformation|AttachComponentToComponent (Variables|/Script/Forgeborn.PlayerCharacter|GetEquippedItem _playercharacter) (Variables|/Script/Engine.Character|GetMesh _playercharacter) "GrinderSocket" "SnapToTarget" "SnapToTarget" "SnapToTarget" true)
            (Variables|/Script/Forgeborn.PlayerCharacter|SetAtGrindingWheel (Variables|Default|GetPlayerCharacter) true)
            (bind _returnvalue (Niagara|SpawnSystematLocation "/Game/AmtosphericFX/FX/NS_Sparks_Mild.NS_Sparks_Mild" (Transformation|GetWorldLocation (Variables|Default|GetArrow)) "0, 0, 0" "1.000000,1.000000,1.000000" false))
            (Variables|Default|SetSparks _returnvalue)
            (Utilities|IsValid (Variables|Default|GetCurrentItem)
              (:Is%20Valid
                _)
              (:Is%20Not%20Valid
                (bind _asbp_item_2 (Utilities|Casting|CastToBP_Item (Variables|/Script/Forgeborn.PlayerCharacter|GetEquippedItem (Variables|Default|GetPlayerCharacter))))
                (Variables|Default|SetCurrentItem _asbp_item_2)))
            (Development|SetHiddeninGame (Variables|/Game/_GAME/Blueprints/Actors/Items/BP_Item.BP_Item_C|GetTempWidget (Variables|Default|GetCurrentItem)) true false)
            (Audio|Components|Audio|FadeIn (Variables|Default|GetAudioComponent) 0.5 1.0 0.0 "Linear" :!class /Script/Engine.AudioComponent))
          (:Tempered
            (goto _label_2))
          (:Sharpened
            (CallFunction|AddEntrytoActionLog (Utilities|Text|FormatText "<Item>{item name}</><Alert> already sharpened!</>" (.Name (Utilities|Struct|BreakItem (Variables|/Script/Forgeborn.ItemBase|GetItem (Variables|Default|GetCurrentItem))))))))))))

(event EventOnMinigameWidgetActivated
  (bind _minigamewidgetinstance (Variables|Default|GetMinigameWidgetInstance))
  (Utilities|IsValid _minigamewidgetinstance
    (:Is%20Valid
      (bind _aswb_minigame_widget (Utilities|Casting|CastToWB_MinigameWidget _minigamewidgetinstance))
      (EventDispatchers|UnbindallEventsfromOnMinigameComplete _aswb_minigame_widget) ; For safety so we don't bind multiple times
      (EventDispatchers|AssignOnMinigameComplete _aswb_minigame_widget (delegate Custom|OnMinigameComplete_Event)))))

(fn ConstructionScript
  (|CallParentFunction))