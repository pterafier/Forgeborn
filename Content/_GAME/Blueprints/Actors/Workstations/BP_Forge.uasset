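; Forge workstation where the player places an accepted equipped item to heat it, then takes it back in hand to cool.
; Interact toggles between adding and removing, blocking adds while locked, with action log entries and sounds.
; Each tick the held item's temperature rises in proportion to its gap from the forge's temperature.
; The forge's Temperature component starts cooling on BeginPlay and drives a widget bar showing rising or cooling.
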(event OnComponentActivated(Amb_Forge_Fire)
  (params (Component :type Actor%20Component%20Object%20Reference) (bReset :type Boolean))
  (bind _amb_forge_fire (Variables|Default|GetAmb_Forge_Fire))
  (Audio|Components|Audio|FadeIn _amb_forge_fire 2.0 1.0 0.0 "Linear" :!class /Script/Engine.AudioComponent)
  (Audio|Components|Audio|SetVolumeMultiplier _amb_forge_fire 1.0 :!class /Script/Engine.AudioComponent))

(event OnComponentDeactivated(Amb_Forge_Fire)
  (params (Component :type Actor%20Component%20Object%20Reference))
  (bind _amb_forge_fire (Variables|Default|GetAmb_Forge_Fire))
  (Audio|Components|Audio|FadeOut _amb_forge_fire 0.0 0.0 "Linear" :!class /Script/Engine.AudioComponent)
  (Audio|Components|Audio|SetVolumeMultiplier _amb_forge_fire 0.0 :!class /Script/Engine.AudioComponent))

(event Custom|OnTemperatureChanged_Event
  (params (Temperature :type Float%20%28single-precision%29))
  (CallFunction|HandleTemperatureChange Temperature))

(event EventBeginPlay
  (|CallParentFunction)
  (CallFunction|SetReferences)
  (EventDispatchers|AssignOnTemperatureChanged (Variables|Default|GetTemperature) (delegate Custom|OnTemperatureChanged_Event))
  (CallFunction|SetTempProgressBar (Variables|/Script/Forgeborn.TemperatureComponent|GetTemperature (Variables|Default|GetTemperature)))
  (Default|SetTempCooling (Variables|Default|GetAs%20WB%20Temperature%20Bar))
  (Class|TemperatureComponent|StartCooling (Variables|Default|GetTemperature))
  (Audio|Components|Audio|Stop (Variables|Default|GetFireWhooshComponent))
  (Components|Activation|Activate (Variables|Default|GetAmb_Forge_Fire) false))

(event EventInteract
  (switch Utilities|FlowControl|Switch|SwitchonEWorkstationAction (Variables|Default|GetWorkstationAction)
    (:Add
      (if (not (Variables|Default|GetisLocked))
        (CallFunction|AddItemtoForge)
        (else
          (CallFunction|AddEntrytoActionLog (Utilities|Text|FormatText "<Workstation>Forge</><Alert> is locked!</>")))))
    (:Remove
      (CallFunction|RemoveItemfromForge))))

(event EventTick
  (params (DeltaSeconds :type Float%20%28single-precision%29))
  (CallFunction|HeatItem DeltaSeconds))

(fn ConstructionScript)

(fn SetTempProgressBar
  (params (Temperature :type Float%20%28double-precision%29))
  (Default|SetPercent (Variables|Default|GetAs%20WB%20Temperature%20Bar) (Math|Float|SafeDivide Temperature (Variables|/Script/Forgeborn.TemperatureComponent|GetMaxTemperature (Variables|Default|GetTemperature)))))

(fn HandleTemperatureChange
  (params (Temperature :type Float%20%28double-precision%29))
  (CallFunction|SetTempProgressBar Temperature)
  (if (and (>= (Variables|/Script/Forgeborn.TemperatureComponent|GetTemperature (Variables|Default|GetTemperature)) (Variables|Default|GetLastTemperature)) (!= (Variables|/Script/Forgeborn.TemperatureComponent|GetTemperature (Variables|Default|GetTemperature)) 0.0))
    (Default|SetTempRising (Variables|Default|GetAs%20WB%20Temperature%20Bar))
    (else
      (Default|SetTempCooling (Variables|Default|GetAs%20WB%20Temperature%20Bar))))
  (Variables|Default|SetLastTemperature Temperature))

(fn AddItemtoForge
  (bind _playercharacter (Variables|Default|GetPlayerCharacter))
  (bind _equippeditem (Variables|/Script/Forgeborn.PlayerCharacter|GetEquippedItem _playercharacter))
  (if (Variables|Default|GetisAcceptingItems)
    (Utilities|IsValid _equippeditem
      (:Is%20Valid
        (if (Utilities|Array|ContainsItem (Variables|Default|GetAcceptableItemIds) (.Id (Utilities|Struct|BreakItem (Variables|/Script/Forgeborn.ItemBase|GetItem _equippeditem))))
          (Audio|Components|Audio|Play (Variables|Default|GetFireWhooshComponent) 0.0)
          (Transformation|DetachFromActor (Variables|/Script/Forgeborn.PlayerCharacter|GetEquippedItem (Variables|Default|GetPlayerCharacter)) "KeepWorld" "KeepWorld" "KeepWorld")
          (Transformation|AttachComponentToComponent (Variables|/Script/Forgeborn.PlayerCharacter|GetEquippedItem (Variables|Default|GetPlayerCharacter)) (Variables|Default|GetAnimationTargetLocation) "None" "SnapToTarget" "SnapToTarget" "SnapToTarget" true)
          (Variables|Default|SetCurrentItem (Variables|/Script/Forgeborn.PlayerCharacter|GetEquippedItem (Variables|Default|GetPlayerCharacter)))
          (Class|PlayerCharacter|SetEquippedItem (Variables|Default|GetPlayerCharacter))
          (CallFunction|SetWorkstationAction "Remove" false)
          (CallFunction|AddEntrytoActionLog (Utilities|Text|FormatText "<Item>{item name}</> added to <Workstation>Forge</>" (.Name (Utilities|Struct|BreakItem (Variables|/Script/Forgeborn.ItemBase|GetItem (Variables|Default|GetCurrentItem))))))
          (Audio|PlaySound2D "/Game/_GAME/Audio/WAVs/Quench_Hit_v1_Cue.Quench_Hit_v1_Cue" 1.0 1.0 0.0 0 0)
          (Audio|Components|Audio|FadeOut (Variables|Default|GetFireWhooshComponent) 0.3 0.0 "Linear" :!class /Script/Engine.AudioComponent)
          (bind _asbp_item (Utilities|Casting|CastToBP_Item (Variables|Default|GetCurrentItem)))
          (Development|SetHiddeninGame (Variables|/Game/_GAME/Blueprints/Actors/Items/BP_Item.BP_Item_C|GetTempWidget _asbp_item) false false))))))

(fn SetReferences
  (bind _aswb_temperature_bar (Utilities|Casting|CastToWB_TemperatureBar (UserInterface|GetWidget (Variables|Default|GetTemperatureWidget))))
  (Variables|Default|SetAs%20WB%20Temperature%20Bar _aswb_temperature_bar))

(fn SetWorkstationAction
  (params (Workstation%20Action :type EWorkstationAction%20Enum :default "None") (Is%20Accepting%20Items :type Boolean))
  (Variables|Default|SetWorkstationAction Workstation%20Action)
  (Variables|Default|SetisAcceptingItems Is%20Accepting%20Items))

(fn RemoveItemfromForge
  (bind _firewhooshcomponent (Variables|Default|GetFireWhooshComponent))
  (if (not (Utilities|IsValid (Variables|/Script/Forgeborn.PlayerCharacter|GetEquippedItem (Variables|Default|GetPlayerCharacter))))
    (Transformation|DetachFromActor (Variables|Default|GetCurrentItem) "KeepWorld" "KeepWorld" "KeepWorld")
    (Transformation|AttachComponentToComponent (Variables|Default|GetCurrentItem) (Variables|/Script/Engine.Character|GetMesh (Variables|Default|GetPlayerCharacter)) "WeaponSocket" "SnapToTarget" "SnapToTarget" "SnapToTarget" true)
    (Class|PlayerCharacter|SetEquippedItem (Variables|Default|GetPlayerCharacter) (Variables|Default|GetCurrentItem))
    (CallFunction|StartCoolingItem)
    (CallFunction|AddEntrytoActionLog (Utilities|Text|FormatText "<Item>{item name}</> removed from <Workstation>Forge</>" (CallFunction|GetCurrentItemName)))
    (Variables|Default|SetCurrentItem 0)
    (CallFunction|SetWorkstationAction "Add" true)
    (Audio|PlaySound2D "/Game/_GAME/Audio/WAVs/Quench_Hit_v1_Cue.Quench_Hit_v1_Cue" 1.0 0.9 0.0 0 0)
    (Audio|Components|Audio|Play _firewhooshcomponent 0.0)
    (Audio|Components|Audio|FadeOut _firewhooshcomponent 1.0 0.0 "Linear" :!class /Script/Engine.AudioComponent)))

(fn HeatItem
  (params (DeltaTime :type Float%20%28double-precision%29))
  (bind _currentitem (Variables|Default|GetCurrentItem))
  (bind _temperaturecomponent (Variables|/Script/Forgeborn.ItemBase|GetTemperatureComponent _currentitem))
  (Utilities|IsValid (Variables|Default|GetCurrentItem)
    (:Is%20Valid
      (bind _output_get (LocalVariables|SetTempDelta (- (Variables|/Script/Forgeborn.TemperatureComponent|GetTemperature (Variables|Default|GetTemperature)) (Variables|/Script/Forgeborn.TemperatureComponent|GetTemperature (Variables|/Script/Forgeborn.ItemBase|GetTemperatureComponent (Variables|Default|GetCurrentItem))))))
      (Variables|/Script/Forgeborn.TemperatureComponent|SetTemperatureChangeAmount _temperaturecomponent (* (* _output_get (LocalVariables|GetHeatingScaleValue)) DeltaTime))
      (Class|TemperatureComponent|StopTemperatureChangeTimer _temperaturecomponent)
      (Class|TemperatureComponent|RaiseTemperature _temperaturecomponent))))

(fn StartCoolingItem
  (bind _currentitem (Variables|Default|GetCurrentItem))
  (bind _temperaturecomponent (Variables|/Script/Forgeborn.ItemBase|GetTemperatureComponent _currentitem))
  (Class|TemperatureComponent|StopTemperatureChangeTimer _temperaturecomponent)
  (Variables|/Script/Forgeborn.TemperatureComponent|SetTemperatureChangeAmount _temperaturecomponent (Variables|/Script/Forgeborn.TemperatureComponent|GetDefaultTemperatureChangeAmount _temperaturecomponent))
  (Class|TemperatureComponent|StartCooling _temperaturecomponent)
  (return))

(fn GetCurrentItemName
  (return (.Name (Utilities|Struct|BreakItem (Variables|/Script/Forgeborn.ItemBase|GetItem (Variables|Default|GetCurrentItem))))))

(fn HideTemperatureWidget
  (params (NewHidden :type Boolean))
  (Development|SetHiddeninGame (Variables|Default|GetTemperatureWidget) NewHidden false))