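; BP_StorageTable is a workstation that stores a single item the player places on it and later takes back.
; Interact switches on WorkstationAction: Add attaches the held item to the table's Arrow, Remove returns it to an empty-handed player's WeaponSocket.
; Each transfer flips the action, logs it and plays a sound.
; It also defines ingot counter and item lookup helpers, which the interaction flow never calls.
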(event EventBeginPlay
  (|CallParentFunction)
  (bind _returnvalue (Actor|GetActorOfClass "/Game/_GAME/Blueprints/Actors/Managers/BP_ResourceManager.BP_ResourceManager_C"))
  (Variables|Default|SetResourceManager _returnvalue)
  (Development|SetHiddeninGame (Variables|Default|GetItemCountWidget) (Variables|Properties|GetHideItemCounter) false))

(event EventInteract
  (bind _playercharacter (Variables|Default|GetPlayerCharacter))
  (bind _equippeditem (Variables|/Script/Forgeborn.PlayerCharacter|GetEquippedItem _playercharacter))
  (switch Utilities|FlowControl|Switch|SwitchonEWorkstationAction (Variables|Default|GetWorkstationAction)
    (:Add
      (Utilities|IsValid _equippeditem
        (:Is%20Valid
          (CallFunction|AddHeldItemtoChest _equippeditem))))
    (:Remove
      (Utilities|IsValid (Variables|/Script/Forgeborn.PlayerCharacter|GetEquippedItem (Variables|Default|GetPlayerCharacter))
        (:Is%20Not%20Valid
          (CallFunction|GrabItemfromTable))))))

(fn ConstructionScript)

(fn AddHeldItemtoChest
  (params (Item :type Item%20Base%20Object%20Reference))
  (Variables|Default|SetCurrentItem Item)
  (Transformation|DetachFromActor Item "KeepWorld" "KeepWorld" "KeepWorld")
  (Transformation|AttachComponentToComponent Item (Variables|Default|GetArrow) "None" "SnapToTarget" "SnapToTarget" "KeepWorld" true)
  (Class|PlayerCharacter|SetEquippedItem (Variables|Default|GetPlayerCharacter))
  (CallFunction|AddEntrytoActionLog (Utilities|Text|FormatText "<Item>{item name}</> added to <Workstation>Table</>" (.Name (Utilities|Struct|BreakItem (Variables|/Script/Forgeborn.ItemBase|GetItem Item)))))
  (Audio|PlaySound2D "/Game/_GAME/Audio/WAVs/Foley_-Forgeborn_2_-_Clothing_4__Cue.Foley_-Forgeborn_2_-_Clothing_4__Cue" 1.0 1.0 0.0 0 0)
  (Variables|Default|SetWorkstationAction "Remove"))

(fn GrabItemfromTable
  (Utilities|IsValid (Variables|Default|GetCurrentItem)
    (:Is%20Valid
      (Transformation|AttachComponentToComponent (Variables|Default|GetCurrentItem) (Variables|/Script/Engine.Character|GetMesh (Variables|Default|GetPlayerCharacter)) "WeaponSocket" "SnapToTarget" "SnapToTarget" "SnapToTarget" true)
      (Class|PlayerCharacter|SetEquippedItem (Variables|Default|GetPlayerCharacter) (Variables|Default|GetCurrentItem))
      (CallFunction|AddEntrytoActionLog (Utilities|Text|FormatText "<Item>{item name}</> removed from <Workstation>Table </>" (.Name (Utilities|Struct|BreakItem (Variables|/Script/Forgeborn.ItemBase|GetItem (Variables|Default|GetCurrentItem))))))
      (Audio|PlaySound2D "/Game/_GAME/Audio/WAVs/Foley_-Forgeborn_2_-_Clothing_4__Cue.Foley_-Forgeborn_2_-_Clothing_4__Cue" 1.0 1.0 0.0 0 0)
      (Variables|Default|SetCurrentItem 0)
      (Variables|Default|SetWorkstationAction "Add"))))

(fn TryDecrementIngotCounter
  (if (> (Variables|Default|GetItemCount) 0)
    (Math|Integer|DecrementInt (Variables|Default|GetItemCount)
      (:%20%20
        (CallFunction|UpdateItemCountText)
        (return true)))
    (else
      (return false))))

(fn IncrementIngotCounter
  (Math|Integer|IncrementInt (Variables|Default|GetItemCount)
    (:%20%20
      (CallFunction|UpdateItemCountText))))

(fn UpdateItemCountText
  (Utilities|IsValid (Variables|Default|GetAs%20WB%20Item%20Counter)
    (:Is%20Valid
      _)
    (:Is%20Not%20Valid
      (bind _aswb_item_counter (Utilities|Casting|CastToWB_ItemCounter (UserInterface|GetWidget (Variables|Default|GetItemCountWidget))))
      (Variables|Default|SetAs%20WB%20Item%20Counter _aswb_item_counter)))
  (Default|UpdateItemText (Variables|Default|GetAs%20WB%20Item%20Counter) (Utilities|Text|ToText(Integer) (Variables|Default|GetItemCount))))

(fn FindItem
  (params (Id :type Integer))
  (bind _returnvalue (Utilities|GetDataTableRow "/Game/_GAME/Data/DT_Items.DT_Items" (Utilities|String|StringToName (Utilities|String|ToString(Integer) Id)))
    (:then
      _)
    (:RowNotFound
      _))
  (return _returnvalue))