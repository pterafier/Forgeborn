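; BP_WorkstationBase is the workstation base actor, providing shared popup labeling, action-log and quality-feedback helpers.
; On BeginPlay it writes ActorName into the interact popup widget's action text.
; AddEntryToActionLog creates a rich text entry and adds it to the player HUD log, lazily resolving and caching the HUD widget.
; PlayFinishedQualitySound plays a 2D completion sound by quality tier, with Fair and Good sharing one.
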(event EventBeginPlay
  (bind _aswb_interact_popup (Utilities|Casting|CastToWB_InteractPopup (UserInterface|GetWidget (Variables|Default|GetPopupWidgetComponent))))
  (Rendering|Components|TextRender|SetText (Variables|/Game/_GAME/UI/Widgets/HUD/Interaction/WB_InteractPopup.WB_InteractPopup_C|GetTXT_ActionText _aswb_interact_popup) (Utilities|Text|FormatText "{workstation}" (Variables|Default|GetActorName))))

(fn ConstructionScript)

(fn AddEntrytoActionLog
  (params (FormattedText :type Text%20%28by%20ref%29))
  (bind _returnvalue (UserInterface|CreateWidget "/Game/_GAME/UI/Widgets/HUD/ActionLog/WB_RichTextEntry.WB_RichTextEntry_C" (Game|GetPlayerController 0)))
  (bind _output_get (LocalVariables|SetNewRichTextWidget _returnvalue))
  (Default|SetRichText _output_get FormattedText)
  (Utilities|IsValid (Variables|Default|GetAs%20WB%20Player%20HUDWidget)
    (:Is%20Valid
      _)
    (:Is%20Not%20Valid
      (bind _aswb_player_hudwidget (Utilities|Casting|CastToWB_PlayerHUDWidget (Variables|/Script/Forgeborn.PlayerHUD|GetPlayerHUDWidget (Variables|/Script/Forgeborn.PlayerControllerBase|GetPlayerHUDActor (Variables|/Script/Forgeborn.PlayerCharacter|GetPlayerControllerBase (Variables|Default|GetPlayerCharacter))))))
      (Variables|Default|SetAs%20WB%20Player%20HUDWidget _aswb_player_hudwidget)))
  (Default|AddChildtoActionLog (Variables|Default|GetAs%20WB%20Player%20HUDWidget) (LocalVariables|GetNewRichTextWidget)))

(fn PlayFinishedQualitySound
  (params (Selection :type EItemQuality%20Enum :default "None"))
  (switch Utilities|FlowControl|Switch|SwitchonEItemQuality Selection
    (:Poor
      (Audio|PlaySound2D "/Game/_GAME/Audio/WAVs/Weapon_Complete_Bad.Weapon_Complete_Bad" 1.0 1.0 0.0 0 0))
    (:Fair
      (Audio|PlaySound2D "/Game/_GAME/Audio/WAVs/Weapon_Complete_Fair_v2_2.Weapon_Complete_Fair_v2_2" 1.0 1.0 0.0 0 0))
    (:Good
      (Audio|PlaySound2D "/Game/_GAME/Audio/WAVs/Weapon_Complete_Fair_v2_2.Weapon_Complete_Fair_v2_2" 1.0 1.0 0.0 0 0))
    (:Excellent
      (Audio|PlaySound2D "/Game/_GAME/Audio/WAVs/Weapon_Complete_Good_v2_2.Weapon_Complete_Good_v2_2" 1.0 1.0 0.0 0 0))
    (:Legendary
      (Audio|PlaySound2D "/Game/_GAME/Audio/WAVs/Weapon_Complete_Excell_v2_1.Weapon_Complete_Excell_v2_1" 1.0 1.0 0.0 0 0))))