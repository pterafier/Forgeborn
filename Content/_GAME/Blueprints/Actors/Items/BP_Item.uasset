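; BP_Item is a forge item actor that heats, cools, transforms, takes damage and breaks based on temperature.
; Temperature component changes update a widget and item state, then either transform the item from DT_Items or mark it ready for shaping.
; Above damage temperature a looping timer drains Quality, and reaching maximum destroys it and notifies the forge.
; DoOnce gates limit HUD action-log messages and sounds to threshold crossings.
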(event Custom|OnTemperatureChanged_Event
  (params (Temperature :type Float%20%28single-precision%29))
  (bind _as_wb_item_temperature (Variables|Default|GetAs%20WB%20Item%20Temperature))
  (bind _item (Variables|Default|GetItem))
  (bind (_id _name _description _transformsafterreachingtargettemperature _targettransformationtemperature _takesdamage _damagetemperature _maxtemperature _transformsinto_datatablerowname) (Utilities|Struct|BreakItem _item))
  (bind _tempalert (Variables|/Game/_GAME/UI/Widgets/HUD/Workstation/WB_ItemTemperature.WB_ItemTemperature_C|GetTempAlert _as_wb_item_temperature))
  (bind _output_get (Variables|Default|SetIncomingTemperature Temperature))
  (CallFunction|UpdateProgressBar _output_get)
  ;[0.15 0.15 0.15 0.5] True if item is hot enough to move to the next stage
  (if (>= (Variables|Default|GetIncomingTemperature) _targettransformationtemperature)
    (if _transformsafterreachingtargettemperature
      (CallFunction|TransformItem _transformsinto_datatablerowname _name)
      (else
        (Default|HideReadyIndicator (Variables|Default|GetAs%20WB%20Item%20Temperature) false)
        (Class|ItemBase|SetItemState "Hot")
        (Utilities|FlowControl|Sequence
          (:then_0
            ;[0.15 0.15 0.15 0.5] True if the item is hot enough to take damage
            (if (>= (Variables|Default|GetIncomingTemperature) _damagetemperature)
              ;[0.15 0.15 0.15 0.5] Break item
              (if (not (CallFunction|IsItematMaxTemp))
                (Utilities|FlowControl|DoOnce false :!label _label
                  (:Completed
                    ;[0.15 0.15 0.15 0.5] Tell player that item is taking damage. Actual damage occurs in DamageItem event. Should play sound there to indicate damage
                    (Variables|Default|SetTemp%20Alert _tempalert)
                    (UserInterface|Animation|PlayAnimation _as_wb_item_temperature _tempalert 0.0 0 "Forward" 1.0 false)
                    (bind _returnvalue (Utilities|Time|SetTimerbyEvent (delegate Custom|DamageItem) 0.25 true))
                    (Variables|Default|SetDamageItemTimerHandle _returnvalue)
                    (CallFunction|AddEntrytoActionLog (Utilities|Text|FormatText "<Item>{item name}</><Alert> is taking heat damage!</>" (.Name (Utilities|Struct|BreakItem (Variables|Default|GetItem)))))
                    (goto _label_2 Reset)))
                (else
                  (Default|SetWorkstationAction (Variables|Default|GetForgeRef) "Add" true)
                  (CallFunction|AddEntrytoActionLog (Utilities|Text|FormatText "<Item>{item name}</><Alert> has broken!</>" (.Name (Utilities|Struct|BreakItem (Variables|Default|GetItem)))))
                  (Audio|PlaySound2D "/Game/_GAME/Audio/WAVs/Anvil_Miss_v2.Anvil_Miss_v2" 1.0 1.0 0.0 0 0)
                  (Actor|DestroyActor)))
              (else
                ;[0.15 0.15 0.15 0.5] Stop damage timer and hide warning indicator
                (Utilities|FlowControl|Sequence
                  (:then_0
                    (goto _label Reset))
                  (:then_1
                    (Default|HideWarningIndicator (Variables|Default|GetAs%20WB%20Item%20Temperature) true)
                    (Utilities|IsValid (Variables|Default|GetTemp%20Alert)
                      (:Is%20Valid
                        (Class|UserWidget|StopAnimation (Variables|Default|GetAs%20WB%20Item%20Temperature) (Variables|Default|GetTemp%20Alert))
                        (Utilities|Time|ClearandInvalidateTimerbyHandle (Variables|Default|GetDamageItemTimerHandle))
                        (Utilities|FlowControl|DoOnce false :!label _label_2
                          (:Completed
                            (CallFunction|AddEntrytoActionLog (Utilities|Text|FormatText "<Item>{item name}</> has stopped taking damage" (.Name (Utilities|Struct|BreakItem (Variables|Default|GetItem))))))))))))))
          (:then_1
            (Utilities|FlowControl|DoOnce false :!label _label_3
              (:Completed
                (CallFunction|AddEntrytoActionLog (Utilities|Text|FormatText "<Item>{item name}</> has reached shaping temperature" _name))
                (Variables|Default|SethasBeenAtShapingTemp true)
                (Audio|PlaySound2D "/Game/_GAME/Audio/WAVs/Hit_Marker_V4_2.Hit_Marker_V4_2" 1.0 1.0 0.0 0 0)))))))
    (else
      (Default|HideReadyIndicator (Variables|Default|GetAs%20WB%20Item%20Temperature) true)
      (Utilities|FlowControl|Sequence
        (:then_0
          (if (Variables|Default|GethasBeenAtShapingTemp)
            (Utilities|FlowControl|DoOnce false :!label _label_4
              (:Completed
                (CallFunction|AddEntrytoActionLog (Utilities|Text|FormatText "<Item>{item name}</> is no longer at shaping temperature" (.Name (Utilities|Struct|BreakItem (Variables|Default|GetItem)))))
                (Variables|Default|SethasBeenAtShapingTemp false)))
            (else
              (goto _label_4 Reset))))
        (:then_1
          (goto _label_3 Reset))))))

(event Custom|DamageItem
  ;[0.15 0.15 0.15 0.5] Tell player that item is taking damage. Actual damage occurs in DamageItem event. Should play sound there to indicate damage
  (Audio|PlaySound2D "/Game/_GAME/Audio/WAVs/Hit_Marker_Layer_Demo.Hit_Marker_Layer_Demo" 1.0 (Math|Random|RandomFloatinRange 0.9 1.1) 0.0 0 0)
  (Variables|Default|SetQuality (- (Variables|Default|GetQuality) (Variables|Default|GetDamagePerTick))))

(event EventBeginPlay
  (EventDispatchers|AssignOnTemperatureChanged (Variables|Default|GetTemperatureComponent) (delegate Custom|OnTemperatureChanged_Event))
  (CallFunction|SetReferences)
  (CallFunction|UpdateProgressBar (Variables|/Script/Forgeborn.TemperatureComponent|GetTemperature (Variables|Default|GetTemperatureComponent)))
  (Default|HideReadyIndicator (Variables|Default|GetAs%20WB%20Item%20Temperature) true)
  (Default|HideWarningIndicator (Variables|Default|GetAs%20WB%20Item%20Temperature) true))

(fn ConstructionScript)

(fn UpdateProgressBar
  (params (NewTemperature :type Float%20%28double-precision%29))
  (bind _as_wb_item_temperature (Variables|Default|GetAs%20WB%20Item%20Temperature))
  (Utilities|IsValid _as_wb_item_temperature
    (:Is%20Valid
      (Default|SetPercent _as_wb_item_temperature (Math|Float|SafeDivide NewTemperature (Variables|/Script/Forgeborn.TemperatureComponent|GetMaxTemperature (Variables|Default|GetTemperatureComponent))))
      (if (and (>= (Variables|/Script/Forgeborn.TemperatureComponent|GetTemperature (Variables|Default|GetTemperatureComponent)) (Variables|Default|GetLastTemperature)) (!= (Variables|/Script/Forgeborn.TemperatureComponent|GetTemperature (Variables|Default|GetTemperatureComponent)) 0.0))
        (Default|SetTempRising (Variables|Default|GetAs%20WB%20Item%20Temperature))
        (if (Utilities|Enum|NotEqual(Enum) (.ForgeState (Utilities|Struct|BreakItem (Variables|Default|GetItem))) "Hot")
          (Class|ItemBase|SetItemState "Heating"))
        (else
          (Default|SetTempCooling (Variables|Default|GetAs%20WB%20Item%20Temperature))
          (Class|ItemBase|SetItemState "Cooling")))
      (Variables|Default|SetLastTemperature NewTemperature))))

(fn TransformItem
  (params (DataTableRowName :type Name) (OldItemName :type Name))
  (bind _returnvalue (Utilities|GetDataTableRow "/Game/_GAME/Data/DT_Items.DT_Items" DataTableRowName)
    (:then
      (Class|ItemBase|SetItem _returnvalue)
      (Components|SkeletalMesh|SetSkeletalMeshAsset (Variables|Default|GetSkeletalMeshComponent) (.Mesh (Utilities|Struct|BreakItem _returnvalue)))
      (Variables|/Script/Forgeborn.TemperatureComponent|SetTemperature (Variables|Default|GetTemperatureComponent) 0.0)
      (Default|SetTempmarkerforShaping (Variables|Default|GetAs%20WB%20Item%20Temperature))
      (Variables|Default|SetItemProgressState "Ingot")
      (CallFunction|AddEntrytoActionLog (Utilities|Text|FormatText "<Item>{old item name}</> successfully smelted into <Item>{new item name}</>" OldItemName (.Name (Utilities|Struct|BreakItem _returnvalue))))
      (Audio|PlaySound2D "/Game/_GAME/Audio/WAVs/Quench_Miss_v1.Quench_Miss_v1" 1.0 1.0 0.0 0 0))))

(fn IsItematMaxTemp
  (return (>= (Variables|Default|GetIncomingTemperature) (Variables|/Script/Forgeborn.TemperatureComponent|GetMaxTemperature (Variables|Default|GetTemperatureComponent)))))

(fn ResetItemTemperature
  (bind _temp_alert (Variables|Default|GetTemp%20Alert))
  (Default|HideReadyIndicator (Variables|Default|GetAs%20WB%20Item%20Temperature) true)
  (Default|HideWarningIndicator (Variables|Default|GetAs%20WB%20Item%20Temperature) true)
  (Variables|/Script/Forgeborn.TemperatureComponent|SetTemperature (Variables|Default|GetTemperatureComponent) 0.0)
  (Default|SetTempCooling (Variables|Default|GetAs%20WB%20Item%20Temperature))
  (Class|ItemBase|SetItemState "Cooling")
  (Default|CallOnTemperatureChanged (Variables|Default|GetTemperatureComponent) 0.0)
  (Utilities|Time|ClearandInvalidateTimerbyHandle (Variables|Default|GetDamageItemTimerHandle))
  (Utilities|IsValid _temp_alert
    (:Is%20Valid
      (Class|UserWidget|StopAnimation (Variables|Default|GetAs%20WB%20Item%20Temperature) _temp_alert))))

(fn AddEntrytoActionLog
  (params (FormattedText :type Text%20%28by%20ref%29))
  (bind _returnvalue (UserInterface|CreateWidget "/Game/_GAME/UI/Widgets/HUD/ActionLog/WB_RichTextEntry.WB_RichTextEntry_C" (Game|GetPlayerController 0)))
  (bind _output_get (LocalVariables|SetNewRichTextWidget _returnvalue))
  (Default|SetRichText _output_get FormattedText)
  (Utilities|IsValid (Variables|Default|GetAs%20WB%20Player%20HUDWidget)
    (:Is%20Valid
      _)
    (:Is%20Not%20Valid
      (bind _aswb_player_hudwidget (Utilities|Casting|CastToWB_PlayerHUDWidget (Variables|/Script/Forgeborn.PlayerHUD|GetPlayerHUDWidget (Variables|/Script/Forgeborn.PlayerControllerBase|GetPlayerHUDActor (Variables|/Script/Forgeborn.PlayerCharacter|GetPlayerControllerBase (Variables|Default|GetPlayerCharacter))))))
      (Variables|Default|SetAs%20WB%20Player%20HUDWidget _aswb_player_hudwidget)))
  (Default|AddChildtoActionLog (Variables|Default|GetAs%20WB%20Player%20HUDWidget) (LocalVariables|GetNewRichTextWidget)))

(fn SetReferences
  (bind _aswb_item_temperature (Utilities|Casting|CastToWB_ItemTemperature (UserInterface|GetWidget (Variables|Default|GetTempWidget))))
  (Variables|Default|SetAs%20WB%20Item%20Temperature _aswb_item_temperature)
  (bind _asplayer_character (Utilities|Casting|CastToPlayerCharacter (Game|GetPlayerCharacter 0)))
  (Variables|Default|SetPlayerCharacter _asplayer_character)
  (bind _returnvalue (Actor|GetActorOfClass "/Game/_GAME/Blueprints/Actors/Workstations/BP_Forge.BP_Forge_C"))
  (Variables|Default|SetForgeRef _returnvalue))

(fn ConfigureItem
  (params (ItemDetails :type Item%20Structure))
  (Components|SkeletalMesh|SetSkeletalMeshAsset (Variables|Default|GetSkeletalMeshComponent) (.Mesh (Utilities|Struct|BreakItem ItemDetails))))