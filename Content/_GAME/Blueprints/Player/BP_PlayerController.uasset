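; Player controller Blueprint that drives the game's menu and HUD widgets through MainWidget's menu stack.
; On begin play it pauses the game and pushes a welcome screen after short delays; a separate event pushes the help menu.
; Input actions fade in the HUD action log, caching the HUD widget on first use, and push or remove the order tracker based on LogMenuOpen, which resets when stacks clear.
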(event Custom|OnStacksCleared_Event
  (Variables|Default|SetLogMenuOpen false))

(event Custom|OpenForgeGuide
  (bind _mainwidget (Variables|Default|GetMainWidget))
  (Utilities|FlowControl|Delay 0.5)
  (Class|MainWidget|PushWidgettoTargetStack _mainwidget (Variables|/Script/Forgeborn.MainWidget|GetMenu_Stack _mainwidget) "/Game/_GAME/UI/Widgets/Menus/WB_HelpMenu.WB_HelpMenu_C" true false false))

(event Input|EnhancedActionEvents|EnhancedInputActionIA_ShowActionLog
  (params (ActionValue :type Boolean) (ElapsedSeconds :type Float%20%28double-precision%29) (TriggeredSeconds :type Float%20%28double-precision%29) (InputAction :type Input%20Action%20Object%20Reference :default "/Game/_GAME/Blueprints/Player/Input/Actions/Gameplay/IA_ShowActionLog.IA_ShowActionLog"))
  (:Started
    (Utilities|IsValid (Variables|Default|GetAs%20WB%20Player%20HUDWidget)
      (:Is%20Valid
        (if (<= (Class|Widget|GetRenderOpacity (Variables|/Game/_GAME/UI/Widgets/HUD/WB_PlayerHUDWidget.WB_PlayerHUDWidget_C|GetWB_ActionLog (Variables|Default|GetAs%20WB%20Player%20HUDWidget))) 0.0)
          (UserInterface|Animation|PlayAnimation (stale _output_get) (Variables|/Game/_GAME/UI/Widgets/HUD/WB_PlayerHUDWidget.WB_PlayerHUDWidget_C|GetFadeInActionLog (stale _output_get)) 0.0 1 "Forward" 1.0 false :!label _label)
          (Default|ResetHideTimer (Variables|Default|GetAs%20WB%20Player%20HUDWidget))))
      (:Is%20Not%20Valid
        (bind _aswb_player_hudwidget (Utilities|Casting|CastToWB_PlayerHUDWidget (Variables|/Script/Forgeborn.PlayerHUD|GetPlayerHUDWidget (Variables|/Script/Forgeborn.PlayerControllerBase|GetPlayerHUDActor (Variables|/Script/Forgeborn.PlayerCharacter|GetPlayerControllerBase (Variables|Default|GetPlayerCharacter))))))
        (bind _output_get (Variables|Default|SetAs%20WB%20Player%20HUDWidget _aswb_player_hudwidget))
        (goto _label)))))

(event Input|EnhancedActionEvents|EnhancedInputActionIA_OpenOrderLog
  (params (ActionValue :type Boolean) (ElapsedSeconds :type Float%20%28double-precision%29) (TriggeredSeconds :type Float%20%28double-precision%29) (InputAction :type Input%20Action%20Object%20Reference :default "/Game/_GAME/Blueprints/Player/Input/Actions/Gameplay/IA_OpenOrderLog.IA_OpenOrderLog"))
  (bind _mainwidget (Variables|Default|GetMainWidget))
  (:Started
    (if (not (Variables|Default|GetLogMenuOpen))
      (bind _returnvalue (Class|MainWidget|PushWidgettoTargetStack _mainwidget (Variables|/Script/Forgeborn.MainWidget|GetMenu_Stack _mainwidget) "/Game/_GAME/UI/Widgets/Menus/CustomerOrder/WB_OrderTracker.WB_OrderTracker_C" true false false))
      (bind _aswb_order_tracker (Utilities|Casting|CastToWB_OrderTracker _returnvalue))
      (Variables|Default|SetAs%20WB%20Order%20Tracker _aswb_order_tracker)
      (else
        (Utilities|IsValid (Variables|Default|GetAs%20WB%20Order%20Tracker)
          (:Is%20Valid
            (Class|MainWidget|RemoveWidget (Variables|Default|GetMainWidget) (Variables|Default|GetAs%20WB%20Order%20Tracker))))))))

(event EventBeginPlay
  (bind _mainwidget (Variables|Default|GetMainWidget))
  (Utilities|FlowControl|Delay 0.1)
  (Game|SetGamePaused true)
  (Utilities|FlowControl|Delay 0.5)
  (EventDispatchers|AssignOnStacksCleared (Variables|Default|GetMainWidget) (delegate Custom|OnStacksCleared_Event))
  (Class|MainWidget|PushWidgettoTargetStack _mainwidget (Variables|/Script/Forgeborn.MainWidget|GetMenu_Stack _mainwidget) "/Game/_GAME/UI/Widgets/Menus/WB_Welcome.WB_Welcome_C" true false false))

(fn ConstructionScript)