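; Player character for a workstation-based smithing game, holding gold and reputation and swinging a hammer at the anvil.
; Left click, right click and spacebar from the controller share one strike event, gated by workstation, whose montage notify spawns impact VFX.
; AddGold and AddReputation update the HUD through a lazily cached widget reference.
; The construction script sockets the hammer mesh, and debug keys spawn customers or attempt rent payment.
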(event Custom|OnLeftClickPressed_Event
  (if (and (Variables|Default|GetCanSwingHammer) (== (Variables|/Script/Forgeborn.PlayerControllerBase|GetCurrentWorkstation (Variables|Default|GetPlayerControllerBase)) (Variables|Default|GetAnvilRef)))
    (Animation|Montage|PlayMontage (Variables|Character|GetMesh) "/Game/_GAME/Assets/Characters/RetargetedAnimations/Anim_Player_Anvil_Strike_Anim_Montage.Anim_Player_Anvil_Strike_Anim_Montage" 1.0 0.0 "None" false
      (:OnNotifyBegin
        (Niagara|SpawnSystematLocation "/Game/HitsImpactsVol1/Particles/NiagaraSystems/NS_HitImpact_v24.NS_HitImpact_v24" (Transformation|GetWorldLocation (Variables|/Game/_GAME/Blueprints/Actors/Workstations/BP_Anvil.BP_Anvil_C|GetVFXLocation (Variables|Default|GetAnvilRef))))))))

(event EventBeginPlay
  (bind _playercontrollerbase (Variables|Default|GetPlayerControllerBase))
  (bind _returnvalue (Actor|GetActorOfClass "/Game/_GAME/Blueprints/Actors/Workstations/BP_Anvil.BP_Anvil_C"))
  (Variables|Default|SetAnvilRef _returnvalue)
  (EventDispatchers|AssignOnLeftClickPressed _playercontrollerbase (delegate Custom|OnLeftClickPressed_Event))
  (EventDispatchers|BindEventtoOnRightClickPressed _playercontrollerbase (delegate Custom|OnLeftClickPressed_Event))
  (EventDispatchers|BindEventtoOnSpacebarPressed _playercontrollerbase (delegate Custom|OnLeftClickPressed_Event)))

(event Input|KeyboardEvents|DebugKey1
  (params (Key :type Key%20Structure :default "None") (ActionValue :type Input%20Action%20Value%20Structure))
  (:Pressed
    (bind _returnvalue (Actor|GetActorOfClass "/Game/_GAME/Blueprints/Actors/AI/BP_SpawnLocation.BP_SpawnLocation_C"))
    (Game|SpawnActorfromClass "/Game/_GAME/Blueprints/AI/BP_Customer.BP_Customer_C" (Transformation|GetActorTransform _returnvalue) "AdjustIfPossibleButAlwaysSpawn" "MultiplyWithRoot" 0 0 0 "None" 0 3e+01 0 0)))

(event Input|KeyboardEvents|DebugKey2
  (params (Key :type Key%20Structure :default "None") (ActionValue :type Input%20Action%20Value%20Structure))
  (:Pressed
    (bind _returnvalue (Actor|GetActorOfClass "/Game/_GAME/Blueprints/Actors/Managers/BP_ScheduleManager.BP_ScheduleManager_C"))
    (Default|TryPayRent _returnvalue)))

(fn ConstructionScript
  (Transformation|AttachComponentToComponent (Variables|Default|GetHammerMesh) (Variables|Character|GetMesh) "GrinderSocket" "SnapToTarget" "SnapToTarget" "SnapToTarget" true))

(fn AddReputation
  (params (AmountToAdd :type Integer))
  (Variables|Default|SetReputation (+ AmountToAdd (Variables|Default|GetReputation)))
  (Utilities|IsValid (Variables|Default|GetAs%20WB%20Player%20HUDWidget)
    (:Is%20Valid
      _)
    (:Is%20Not%20Valid
      (bind _aswb_player_hudwidget (Utilities|Casting|CastToWB_PlayerHUDWidget (Variables|/Script/Forgeborn.PlayerHUD|GetPlayerHUDWidget (Variables|/Script/Forgeborn.PlayerControllerBase|GetPlayerHUDActor (Variables|Default|GetPlayerControllerBase)))))
      (Variables|Default|SetAs%20WB%20Player%20HUDWidget _aswb_player_hudwidget)))
  (Default|UpdateReputation (Variables|/Game/_GAME/UI/Widgets/HUD/WB_PlayerHUDWidget.WB_PlayerHUDWidget_C|GetWB_Resources (Variables|Default|GetAs%20WB%20Player%20HUDWidget)) (Variables|Default|GetReputation)))

(fn AddGold
  (params (AmountToAdd :type Integer))
  (Variables|Default|SetGold (+ AmountToAdd (Variables|Default|GetGold)))
  (Utilities|IsValid (Variables|Default|GetAs%20WB%20Player%20HUDWidget)
    (:Is%20Valid
      _)
    (:Is%20Not%20Valid
      (bind _aswb_player_hudwidget (Utilities|Casting|CastToWB_PlayerHUDWidget (Variables|/Script/Forgeborn.PlayerHUD|GetPlayerHUDWidget (Variables|/Script/Forgeborn.PlayerControllerBase|GetPlayerHUDActor (Variables|Default|GetPlayerControllerBase)))))
      (Variables|Default|SetAs%20WB%20Player%20HUDWidget _aswb_player_hudwidget)))
  (Default|UpdateGold (Variables|/Game/_GAME/UI/Widgets/HUD/WB_PlayerHUDWidget.WB_PlayerHUDWidget_C|GetWB_Resources (Variables|Default|GetAs%20WB%20Player%20HUDWidget)) (Variables|Default|GetGold)))