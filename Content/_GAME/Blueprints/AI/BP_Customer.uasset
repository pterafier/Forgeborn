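; Forge customer AI that walks to the order window on spawn and leaves to be destroyed if its timed wait, shown on a progress bar, expires.
; First interaction generates a random order with week-weighted ore tiers, weekday due date and summed item-value reward for the order widget.
; Accepted orders register with the ScheduleManager and send the customer to wait.
; PickupOrder retries until the pickup window is free; later interactions open the pickup widget.
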(event Custom|LeaveOrderWindowAndDie
  (bind _deathlocation (Variables|LocationActors|GetDeathLocation))
  (Default|AddEntrytoActionLog (Variables|/Game/_GAME/Blueprints/Actors/Managers/BP_ScheduleManager.BP_ScheduleManager_C|GetForgeRef (Variables|Default|GetScheduleManager)) (Utilities|Text|MakeLiteralText "A customer has left"))
  (Variables|Default|SetCanInteract false)
  (Variables|Default|SetAtOrderWindow false)
  (Development|SetHiddeninGame (Variables|Default|GetProgressBar) true false)
  (Utilities|IsValid _deathlocation
    (:Is%20Valid
      (AI|AIMoveTo self (Transformation|GetActorLocation _deathlocation) _deathlocation 5.0 false
        (:OnSuccess
          _)
        (:OnFail
          (Components|Movement|StopMovementImmediately (Variables|Character|GetCharacterMovement))))
      (Utilities|FlowControl|Delay 5.0)
      (Actor|DestroyActor))))

(event Custom|UpdateProgressBar
  (Default|SetPercent (Variables|Default|GetTimeProgressBar) (Math|Float|SafeDivide (Utilities|Time|GetTimerRemainingTimebyHandle (Variables|TimerHandles|GetWaitTimeTimerHandle)) (Variables|Default|GetWaitTime))))

(event Custom|MoveToWaitingLocation
  (Variables|Default|SetAtOrderWindow false)
  (AI|AIMoveTo self (Transformation|GetActorLocation (Variables|LocationActors|GetWaitLocation)) 0 1.0 false))

(event Custom|PickupOrder
  (bind _pickuplocation (Variables|LocationActors|GetPickupLocation))
  (if (not (Variables|/Game/_GAME/Blueprints/Actors/AI/BP_PickupLocation.BP_PickupLocation_C|GetisOccupied _pickuplocation)) :!label _label
    (Variables|Default|SetOnTheWayToPickupOrder true)
    (AI|AIMoveTo self (Transformation|GetActorLocation _pickuplocation) 0 1.0 false
      (:OnSuccess
        (Default|AddEntrytoActionLog (Variables|/Game/_GAME/Blueprints/Actors/Managers/BP_ScheduleManager.BP_ScheduleManager_C|GetForgeRef (Variables|Default|GetScheduleManager)) (Utilities|Text|MakeLiteralText "A customer has arrived at the pickup window"))
        (Audio|PlaySound2D "/Game/_GAME/Audio/WAVs/SC_CustomerGreetingv2.SC_CustomerGreetingv2" 1.0 1.0 0.0 0 0)
        (Audio|PlaySound2D "/Game/_GAME/Audio/WAVs/Coin_Earned_v1.Coin_Earned_v1" 1.0 1.0 0.0 0 0)))
    (else
      (Utilities|FlowControl|Delay 1e+01)
      (goto _label))))

(event EventBeginPlay
  (bind _orderlocation (Variables|LocationActors|GetOrderLocation))
  (CallFunction|SetReferences)
  (Variables|Default|SetAtOrderWindow true)
  (AI|AIMoveTo self (Transformation|GetActorLocation _orderlocation) _orderlocation 1.0 false
    (:OnSuccess
      (Development|SetHiddeninGame (Variables|Default|GetProgressBar) false false)
      (bind _returnvalue (Utilities|Time|SetTimerbyEvent (delegate Custom|LeaveOrderWindowAndDie) (Variables|Default|GetWaitTime)))
      (Variables|TimerHandles|SetWaitTimeTimerHandle _returnvalue)
      (bind _returnvalue_2 (Utilities|Time|SetTimerbyEvent (delegate Custom|UpdateProgressBar) 0.1 true))
      (Variables|TimerHandles|SetProgressBarTimerHandle _returnvalue_2)
      (Default|AddEntrytoActionLog (Variables|/Game/_GAME/Blueprints/Actors/Managers/BP_ScheduleManager.BP_ScheduleManager_C|GetForgeRef (Variables|Default|GetScheduleManager)) (Utilities|Text|MakeLiteralText "A customer has arrived at the order window"))
      (Audio|PlaySound2D "/Game/_GAME/Audio/WAVs/SC_CustomerGreetingv2.SC_CustomerGreetingv2" 1.0 1.0 0.0 0 0)
      (Audio|PlaySound2D "/Game/_GAME/Audio/WAVs/Coin_Misc_v1.Coin_Misc_v1" 1.0 1.0 0.0 0 0))))

(event EventInteract
  (bind _as_player_controller_base (Variables|Default|GetAs%20Player%20Controller%20Base))
  (bind _mainwidget (Variables|/Script/Forgeborn.PlayerControllerBase|GetMainWidget _as_player_controller_base))
  (if (Variables|Default|GetCanInteract)
    (if (not (Variables|Default|GetisPickingUpOrder))
      (CallFunction|CreateOrderPrompt)
      (Utilities|Time|ClearandInvalidateTimerbyHandle (Variables|TimerHandles|GetProgressBarTimerHandle))
      (Utilities|Time|ClearandInvalidateTimerbyHandle (Variables|TimerHandles|GetWaitTimeTimerHandle))
      (Development|SetHiddeninGame (Variables|Default|GetProgressBar) true false)
      (Variables|Default|SetisPickingUpOrder true)
      (else
        (bind _returnvalue (Class|MainWidget|PushWidgettoTargetStack _mainwidget (Variables|/Script/Forgeborn.MainWidget|GetMenu_Stack _mainwidget) "/Game/_GAME/UI/Widgets/Menus/CustomerOrder/WB_CustomerPickup.WB_CustomerPickup_C" true false false))
        (bind _aswb_customer_pickup (Utilities|Casting|CastToWB_CustomerPickup _returnvalue))
        (bind _output_get (Variables|/Game/_GAME/UI/Widgets/Menus/CustomerOrder/WB_CustomerPickup.WB_CustomerPickup_C|SetGeneratedOrder _aswb_customer_pickup (Variables|Default|GetCustomerOrder)))
        (Variables|/Game/_GAME/UI/Widgets/Menus/CustomerOrder/WB_CustomerPickup.WB_CustomerPickup_C|SetOwningCustomer _aswb_customer_pickup self)
        (Rendering|Components|TextRender|SetText (Variables|/Game/_GAME/UI/Widgets/Menus/CustomerOrder/WB_CustomerPickup.WB_CustomerPickup_C|GetTXT_OrderDuration _aswb_customer_pickup) (Utilities|Text|FormatText "Picking up order: {order number}" (.OrderId (Utilities|Struct|BreakOrderDetails _output_get))))))))

(fn ConstructionScript)

(fn SetReferences
  (bind _returnvalue (Actor|GetActorOfClass "/Game/_GAME/Blueprints/Actors/AI/BP_OrderLocation.BP_OrderLocation_C"))
  (Variables|LocationActors|SetOrderLocation _returnvalue)
  (bind _returnvalue_2 (Actor|GetActorOfClass "/Game/_GAME/Blueprints/Actors/AI/BP_PickupLocation.BP_PickupLocation_C"))
  (Variables|LocationActors|SetPickupLocation _returnvalue_2)
  (bind _returnvalue_3 (Actor|GetActorOfClass "/Game/_GAME/Blueprints/Actors/AI/BP_SpawnLocation.BP_SpawnLocation_C"))
  (Variables|LocationActors|SetSpawnLocation _returnvalue_3)
  (bind _aswb_time_progress_bar (Utilities|Casting|CastToWB_TimeProgressBar (UserInterface|GetWidget (Variables|Default|GetProgressBar))))
  (Variables|Default|SetTimeProgressBar _aswb_time_progress_bar)
  (bind _returnvalue_4 (Actor|GetActorOfClass "/Game/_GAME/Blueprints/Actors/Managers/BP_ScheduleManager.BP_ScheduleManager_C"))
  (Variables|Default|SetScheduleManager _returnvalue_4)
  (bind _asplayer_controller_base (Utilities|Casting|CastToPlayerControllerBase (Game|GetPlayerController 0)))
  (Variables|Default|SetAs%20Player%20Controller%20Base _asplayer_controller_base)
  (bind _returnvalue_5 (Actor|GetActorOfClass "/Game/_GAME/Blueprints/Actors/AI/BP_WaitLocation.BP_WaitLocation_C"))
  (Variables|LocationActors|SetWaitLocation _returnvalue_5)
  (bind _returnvalue_6 (Actor|GetActorOfClass "/Game/_GAME/Blueprints/Actors/AI/BP_DeathLocation.BP_DeathLocation_C"))
  (Variables|LocationActors|SetDeathLocation _returnvalue_6))

(fn GenerateOrder
  (Utilities|Array|Clear (Variables|Default|GetDesiredItemIds))
  (bind _output_get (Variables|Default|SetOrderDuration (Math|Random|RandomIntegerinRange (LocalVariables|GetMinDays) (LocalVariables|GetMaxDays))))
  (LocalVariables|SetMaxOrderSize (Math|Integer|Clamp(Integer) (* _output_get 2) 1 3))
  (bind _output_get_2 (Variables|Default|SetOrderSize (Math|Random|RandomIntegerinRange 1 (LocalVariables|GetMaxOrderSize))))
  (for _index (range 1 _output_get_2)
    (bind _ore (CallFunction|GenerateOreSelection))
    (Utilities|Array|Add (LocalVariables|GetOreTypes) _ore))
  (for _array_element (LocalVariables|GetOreTypes)
    (switch Utilities|FlowControl|Switch|SwitchonEOreTypes _array_element
      (:Iron
        (Utilities|Array|Add (Variables|Default|GetDesiredItemIds) (.OutItem (Utilities|Array|Random (Variables|Default|GetIronOreIds)))))
      (:Titanium
        (Utilities|Array|Add (Variables|Default|GetDesiredItemIds) (.OutItem (Utilities|Array|Random (Variables|Default|GetTitaniumOreIds)))))
      (:Steel
        (Utilities|Array|Add (Variables|Default|GetDesiredItemIds) (.OutItem (Utilities|Array|Random (Variables|Default|GetSteelOreIds)))))
      (:Viridium
        (Utilities|Array|Add (Variables|Default|GetDesiredItemIds) (.OutItem (Utilities|Array|Random (Variables|Default|GetViridiumOreIds)))))))
  (bind _day (CallFunction|ConvertDueDatetoDayName (Variables|Default|GetOrderDuration)))
  (bind _reward (CallFunction|CalculateGoldReward))
  (bind _orderid (Default|GenerateOrderId (Variables|Default|GetScheduleManager)))
  (return (Utilities|Struct|MakeOrderDetails _orderid _day (Variables|Default|GetDesiredItemIds) self _reward)))

(fn GenerateOreSelection
  (switch int (Math|Integer|Clamp(Integer) (+ (Variables|/Game/_GAME/Blueprints/Actors/Managers/BP_ScheduleManager.BP_ScheduleManager_C|GetCurrentWeek (Variables|Default|GetScheduleManager)) (Math|Random|RandomIntegerinRange -3 3)) 0 3)
    (:0
      (return "Iron"))
    (:1
      (return "Steel"))
    (:2
      (return "Titanium"))
    (:3
      (return "Viridium"))))

(fn AddOrdertoScheduleManager
  (params (OrderToAdd :type Order%20Details%20Structure%20%28by%20ref%29))
  (Utilities|Array|Add (Variables|/Script/Forgeborn.ScheduleManager|GetActiveOrders (Variables|Default|GetScheduleManager)) OrderToAdd)
  (Default|AddEntrytoActionLog (Variables|/Game/_GAME/Blueprints/Actors/Managers/BP_ScheduleManager.BP_ScheduleManager_C|GetForgeRef (Variables|Default|GetScheduleManager)) (Utilities|Text|FormatText "<Perfect>Order accepted!</> Press TAB for details"))
  (CallFunction|MovetoWaitingLocation))

(fn ConvertDueDatetoDayName
  (params (OrderDuration :type Integer))
  (switch int (+ (.Index (Default|GetDayOftheWeek (Variables|/Game/_GAME/Blueprints/Actors/Managers/BP_ScheduleManager.BP_ScheduleManager_C|GetUDS (Variables|Default|GetScheduleManager)))) OrderDuration)
    (:0
      (return "Monday"))
    (:1
      (return "Tuesday"))
    (:2
      (return "Wednesday"))
    (:3
      (return "Thursday"))
    (:4
      (return "Friday"))
    (:5
      (return "Saturday"))
    (:6
      (return "Sunday"))))

(fn GenerateOrderIcons
  (Utilities|Array|Clear (Variables|Default|GetGeneratedOrderIcons))
  (for _array_element (Variables|Default|GetDesiredItemIds)
    (bind _returnvalue (Utilities|GetDataTableRow "/Game/_GAME/Data/DT_Items.DT_Items" (Utilities|String|StringToName (Utilities|String|ToString(Integer) _array_element)))
      (:then
        (bind _returnvalue_2 (UserInterface|CreateWidget "/Game/_GAME/UI/Widgets/Menus/CustomerOrder/WB_OrderIcon.WB_OrderIcon_C" (Variables|Default|GetAs%20Player%20Controller%20Base)))
        (Default|ConfigureWidget _returnvalue_2 (Utilities|Text|ToText(Name) (.Name (Utilities|Struct|BreakItem _returnvalue))) (.Icon (Utilities|Struct|BreakItem _returnvalue)))
        (Utilities|Array|Add (Variables|Default|GetGeneratedOrderIcons) _returnvalue_2)
        (Development|PrintString (Utilities|String|ToString(Text) (Utilities|Text|ToText(Name) (.Name (Utilities|Struct|BreakItem _returnvalue))))))))
  (return (Variables|Default|GetGeneratedOrderIcons)))

(fn CreateOrderPrompt
  (bind _as_player_controller_base (Variables|Default|GetAs%20Player%20Controller%20Base))
  (bind _mainwidget (Variables|/Script/Forgeborn.PlayerControllerBase|GetMainWidget _as_player_controller_base))
  (bind _order (CallFunction|GenerateOrder))
  (Variables|Default|SetCustomerOrder _order)
  (CallFunction|GenerateOrderIcons)
  (bind _returnvalue (Class|MainWidget|PushWidgettoTargetStack _mainwidget (Variables|/Script/Forgeborn.MainWidget|GetMenu_Stack _mainwidget) "/Game/_GAME/UI/Widgets/Menus/CustomerOrder/WB_CustomerOrder.WB_CustomerOrder_C" true false false))
  (bind _aswb_customer_order (Utilities|Casting|CastToWB_CustomerOrder _returnvalue))
  (Widget|Panel|ClearChildren (Variables|/Game/_GAME/UI/Widgets/Menus/CustomerOrder/WB_CustomerOrder.WB_CustomerOrder_C|GetHB_OrderIconsBox _aswb_customer_order))
  (for _array_element (Variables|Default|GetGeneratedOrderIcons)
    (Default|AddChildtoBox _aswb_customer_order _array_element))
  (Utilities|FlowControl|Sequence
    (:then_0
      (Default|SetDuration _aswb_customer_order (Variables|Default|GetOrderDuration))
      (Default|SetReward _aswb_customer_order (.GoldReward (Utilities|Struct|BreakOrderDetails (Variables|Default|GetCustomerOrder)))))
    (:then_1
      (Variables|/Game/_GAME/UI/Widgets/Menus/CustomerOrder/WB_CustomerOrder.WB_CustomerOrder_C|SetGeneratedOrder _aswb_customer_order (Variables|Default|GetCustomerOrder)))
    (:then_2
      (Variables|/Game/_GAME/UI/Widgets/Menus/CustomerOrder/WB_CustomerOrder.WB_CustomerOrder_C|SetOwningCustomer _aswb_customer_order self))))

(fn CalculateGoldReward
  (for _array_element (Variables|Default|GetDesiredItemIds)
    (bind _returnvalue (Utilities|GetDataTableRow "/Game/_GAME/Data/DT_Items.DT_Items" (Utilities|String|StringToName (Utilities|String|ToString(Integer) _array_element)))
      (:then
        (LocalVariables|SetGoldReward (+ (LocalVariables|GetGoldReward) (.BaseValue (Utilities|Struct|BreakItem _returnvalue)))))))
  (return (LocalVariables|GetGoldReward)))