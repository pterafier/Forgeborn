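; Main menu player controller that builds the menu UI and applies the player's audio volume settings on BeginPlay.
; It creates WB_MainWidget, adds it to the viewport and pushes WB_MainMenu onto that widget's menu stack.
; It then reads master, music, effects and ambient volumes from the audio subsystem, applying each as a sound class override on its own pushed sound mix.
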(event EventBeginPlay
  (bind _returnvalue (UserInterface|CreateWidget "/Game/_GAME/UI/Widgets/WB_MainWidget.WB_MainWidget_C" self))
  (bind _output_get (Variables|Default|SetMainWidgetRef _returnvalue))
  (UserInterface|Viewport|AddtoViewport _output_get 0)
  (Class|MainWidget|PushWidgettoTargetStack (Variables|Default|GetMainWidgetRef) (Variables|/Script/Forgeborn.MainWidget|GetMenu_Stack (Variables|Default|GetMainWidgetRef)) "/Game/_GAME/UI/Widgets/Menus/WB_MainMenu.WB_MainMenu_C" true false false)
  (Audio|SetSoundMixClassOverride "/Game/_GAME/Audio/AudioData/SCM_Master.SCM_Master" "/Engine/EngineSounds/Master.Master" (Variables|/Script/Forgeborn.AudioSubsystem|GetMasterVolume (Subsystems|GetAudioSubsystem)) 1.0 0.0 true)
  (Audio|PushSoundMixModifier "/Game/_GAME/Audio/AudioData/SCM_Master.SCM_Master")
  (Audio|SetSoundMixClassOverride "/Game/_GAME/Audio/AudioData/SCM_Music.SCM_Music" "/Engine/EngineSounds/Music.Music" (Variables|/Script/Forgeborn.AudioSubsystem|GetMusicVolume (Subsystems|GetAudioSubsystem)) 1.0 0.0 true)
  (Audio|PushSoundMixModifier "/Game/_GAME/Audio/AudioData/SCM_Music.SCM_Music")
  (Audio|SetSoundMixClassOverride "/Game/_GAME/Audio/AudioData/SCM_SFX.SCM_SFX" "/Engine/EngineSounds/SFX.SFX" (Variables|/Script/Forgeborn.AudioSubsystem|GetSoundEffectsVolume (Subsystems|GetAudioSubsystem)) 1.0 0.0 true)
  (Audio|PushSoundMixModifier "/Game/_GAME/Audio/AudioData/SCM_SFX.SCM_SFX")
  (Audio|SetSoundMixClassOverride "/Game/_GAME/Audio/AudioData/SCM_Ambient.SCM_Ambient" "/Game/_GAME/Audio/AudioData/Ambient.Ambient" (Variables|/Script/Forgeborn.AudioSubsystem|GetAmbientSoundsVolume (Subsystems|GetAudioSubsystem)) 1.0 0.0 true)
  (Audio|PushSoundMixModifier "/Game/_GAME/Audio/AudioData/SCM_Ambient.SCM_Ambient"))

(fn ConstructionScript)